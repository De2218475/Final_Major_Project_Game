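; Chess board actor that builds a configurable, centred grid of tile meshes and spawns test pieces on clicked tiles.
; The construction script creates green-to-blue tinted tiles, storing each tile's state, grid position, mesh and occupant in an index-keyed TileMap.
; Clicking matches the cursor-hit component to a tile and records the spawned piece there.
; RegenerateTiles rebuilds meshes while keeping state, trims surplus tiles with their pawns, and repositions the rest.
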(event EventBeginPlay)

(event MouseInput|EventActorOnClicked
  (params (ButtonPressed :type Key%20Structure :default "None"))
  (CallFunction|AddPawn))

(fn ConstructionScript
  (CallFunction|SpawnInitialTiles))

(fn CalculateTilePos
  (Variables|Default|SettilePos (Math|Vector|MakeVector (/ (- (* (/ (Variables|Default|GetIndex) (Variables|Default|GetboardCollumnLength)) (+ (Variables|Default|GettileSize) (Variables|Default|GettileSpacing))) (* (/ (- (Variables|Default|GetboardRowLength) 1) 2) (+ (Variables|Default|GettileSize) (Variables|Default|GettileSpacing)))) -1.0) (- (* (Math|Integer|%(Integer) (Variables|Default|GetIndex) (Variables|Default|GetboardCollumnLength)) (+ (Variables|Default|GettileSize) (Variables|Default|GettileSpacing))) (* (/ (- (Variables|Default|GetboardCollumnLength) 1) 2) (+ (Variables|Default|GettileSize) (Variables|Default|GettileSpacing)))) 0.0))
  (return (Math|Vector2D|MakeVector2D (Math|Conversions|ToFloat(Integer) (/ (Variables|Default|GetIndex) (Variables|Default|GetboardCollumnLength))) (Math|Conversions|ToFloat(Integer) (Math|Integer|%(Integer) (Variables|Default|GetIndex) (Variables|Default|GetboardCollumnLength))))))

(fn SpawnInitialTiles
  (for _index (range 0 (- (* (Variables|Default|GetboardCollumnLength) (Variables|Default|GetboardRowLength)) 1))
    (Variables|Default|SetIndex _index)
    (bind _tile2dpos (CallFunction|CalculateTilePos))
    (LocalVariables|SetTile2dPos _tile2dpos)
    (bind _returnvalue (AddComponent|AddStaticMeshComponent false (Math|Transform|MakeTransform (Variables|Default|GettilePos) "0, 0, 0" (Math|Conversions|ToVector(Float) (/ (Variables|Default|GettileSize) 1e+02)))))
    (LocalVariables|SetstaticMeshCompRef _returnvalue)
    (Transformation|AttachComponentToComponent (LocalVariables|GetstaticMeshCompRef) (Variables|Default|GetDefaultSceneRoot) "None" "KeepRelative" "KeepRelative" "KeepRelative" true)
    (bind _returnvalue_2 (Rendering|Material|CreateDynamicMaterialInstance (LocalVariables|GetstaticMeshCompRef) 0 "/Game/MyContent/Materials/MAT_DebugMaterial.MAT_DebugMaterial" "None" :!class /Script/Engine.PrimitiveComponent))
    (Rendering|Material|SetVectorParameterValue _returnvalue_2 "Colour" (Math|Color|Lerp(LinearColor) (Utilities|Struct|MakeLinearColor 0.0 1.0 0.0 1.0) (Utilities|Struct|MakeLinearColor 0.0 0.0 1.0 1.0) (/ (Variables|Default|GetIndex) (- (* (Variables|Default|GetboardCollumnLength) (Variables|Default|GetboardRowLength)) 1))) :!class /Script/Engine.MaterialInstanceDynamic)
    (Utilities|Map|Add (Variables|Default|GettileMap) (Variables|Default|GetIndex) (Utilities|Struct|MakeStr_BoardTileStructure true true 0 (LocalVariables|GetTile2dPos) (LocalVariables|GetstaticMeshCompRef)))))

(fn SortTileElements
  (LocalVariables|Setn (Utilities|Map|Length (Variables|Default|GettileMap)))
  (for _index (range 0 (- (LocalVariables|Getn) 1))
    (LocalVariables|Seti _index)
    (for _index_2 (range 0 (Utilities|Operators|Subtract (LocalVariables|Getn) 1 (LocalVariables|Geti)))
      (LocalVariables|Setj _index_2)
      (bind _keys (Utilities|Map|Keys (Variables|Default|GettileMap)))
      (if (> (Utilities|Array|Get(acopy) _keys (LocalVariables|Getj)) (Utilities|Array|Get(acopy) _keys (+ (LocalVariables|Getj) 1)))
        (bind _keys_2 (Utilities|Map|Keys (Variables|Default|GettileMap)))
        (Utilities|Array|Swap _keys_2 (LocalVariables|Getj) (+ (LocalVariables|Getj) 1)))))
  (Utilities|Map|Clear (Variables|Default|GettempTileMap))
  (bind _keys_3 (Utilities|Map|Keys (Variables|Default|GettileMap)))
  (for (_array_element _array_index) _keys_3
    (Utilities|Map|Add (Variables|Default|GettempTileMap) _array_index (.Value (Utilities|Map|Find (Variables|Default|GettileMap) _array_element))))
  (Utilities|Map|Clear (Variables|Default|GettileMap))
  (bind _keys_4 (Utilities|Map|Keys (Variables|Default|GettempTileMap)))
  (for (_array_element_2 _array_index_2) _keys_4
    (Utilities|Map|Add (Variables|Default|GettileMap) _array_index_2 (.Value (Utilities|Map|Find (Variables|Default|GettempTileMap) _array_element_2)))))

(fn AddPawn
  (bind _returnvalue (Game|GetPlayerController 0))
  (bind _hitresult (Game|Player|GetHitResultUnderCursorbyChannel _returnvalue "TraceTypeQuery1" true))
  (bind _values (Utilities|Map|Values (Variables|Default|GettileMap)))
  (for (_array_element _array_index) _values
    (if (== (.tilecomponentref _array_element) (.hitcomponent _hitresult))
      (bind _returnvalue_2 (Game|SpawnActorfromClass "/Game/MyContent/Pawns/BP_TestChessPiece.BP_TestChessPiece_C" (Math|Transform|MakeTransform (Transformation|GetWorldLocation (.hitcomponent _hitresult)) "0, 0, 0" "1.000000,1.000000,1.000000") "AdjustIfPossibleButAlwaysSpawn" "MultiplyWithRoot" 0 0))
      (Utilities|Map|Add (Variables|Default|GettileMap) _array_index (Utilities|Struct|MakeStr_BoardTileStructure (.istileactive _array_element) (.istilefree _array_element) _returnvalue_2 (.2dtilepos _array_element) (.tilecomponentref _array_element))))))

(fn RegenerateTiles
  (bind _tilemap (Variables|Default|GettileMap))
  (bind _tilemap_2 (Variables|Default|GettileMap))
  (bind _returnvalue (Utilities|Map|Length _tilemap_2))
  (bind _returnvalue_2 (- _returnvalue 1))
  (bind _value (Utilities|Map|Find _tilemap_2 _returnvalue_2))
  (for _index (range 0 (- (Utilities|Map|Length (Variables|Default|GettileMap)) 1))
    (Variables|Default|SetIndex _index)
    (Utilities|IsValid (.tilecomponentref (.Value (Utilities|Map|Find (Variables|Default|GettileMap) (Variables|Default|GetIndex))))
      (:Is%20Valid
        (Components|DestroyComponent (.tilecomponentref (.Value (Utilities|Map|Find (Variables|Default|GettileMap) (Variables|Default|GetIndex))))))
      (:Is%20Not%20Valid
        (Development|PrintString "Invalid Tile"))))
  (for _index_2 (range 0 (- (* (Variables|Default|GetboardCollumnLength) (Variables|Default|GetboardRowLength)) 1))
    (Variables|Default|SetIndex _index_2)
    (bind _tile2dpos (CallFunction|CalculateTilePos))
    (LocalVariables|SetTile2dPos _tile2dpos)
    (bind _returnvalue_3 (AddComponent|AddStaticMeshComponent false (Math|Transform|MakeTransform (Variables|Default|GettilePos) "0, 0, 0" (Math|Conversions|ToVector(Float) (/ (Variables|Default|GettileSize) 1e+02)))))
    (LocalVariables|SetstaticMeshCompRef _returnvalue_3)
    (Transformation|AttachComponentToComponent (LocalVariables|GetstaticMeshCompRef) (Variables|Default|GetDefaultSceneRoot) "None" "KeepRelative" "KeepRelative" "KeepRelative" true)
    (bind _returnvalue_4 (Rendering|Material|CreateDynamicMaterialInstance (LocalVariables|GetstaticMeshCompRef) 0 "/Game/MyContent/Materials/MAT_DebugMaterial.MAT_DebugMaterial" "None" :!class /Script/Engine.PrimitiveComponent))
    (Rendering|Material|SetVectorParameterValue _returnvalue_4 "Colour" (Math|Color|Lerp(LinearColor) (Utilities|Struct|MakeLinearColor 0.0 1.0 0.0 1.0) (Utilities|Struct|MakeLinearColor 0.0 0.0 1.0 1.0) (/ (Variables|Default|GetIndex) (- (* (Variables|Default|GetboardCollumnLength) (Variables|Default|GetboardRowLength)) 1))) :!class /Script/Engine.MaterialInstanceDynamic)
    (Utilities|Map|Add _tilemap (Variables|Default|GetIndex) (Utilities|Struct|MakeStr_BoardTileStructure (.istileactive (.Value (Utilities|Map|Find _tilemap (Variables|Default|GetIndex)))) (.istilefree (.Value (Utilities|Map|Find _tilemap (Variables|Default|GetIndex)))) (.occupiedpawn (.Value (Utilities|Map|Find _tilemap (Variables|Default|GetIndex)))) (LocalVariables|GetTile2dPos) (LocalVariables|GetstaticMeshCompRef))))
  (CallFunction|SortTileElements)
  (while (> (- (Utilities|Map|Length (Variables|Default|GettileMap)) 1) (- (* (Variables|Default|GetboardCollumnLength) (Variables|Default|GetboardRowLength)) 1))
    (Utilities|IsValid (.occupiedpawn _value)
      (:Is%20Valid
        (Actor|DestroyActor (.occupiedpawn _value)))
      (:Is%20Not%20Valid
        _))
    (Utilities|Map|Remove (Variables|Default|GettileMap) (- (Utilities|Map|Length (Variables|Default|GettileMap)) 1)))
  (CallFunction|RepositionPawns))

(fn DeleteAllTiles
  (CallFunction|SortTileElements)
  (for _index (range 0 (- (* (Variables|Default|GetboardCollumnLength) (Variables|Default|GetboardRowLength)) 1))
    (Variables|Default|SetIndex _index)
    (Utilities|IsValid (.tilecomponentref (.Value (Utilities|Map|Find (Variables|Default|GettileMap) (Variables|Default|GetIndex))))
      (:Is%20Valid
        (Components|DestroyComponent (.tilecomponentref (.Value (Utilities|Map|Find (Variables|Default|GettileMap) (Variables|Default|GetIndex)))))
        (Utilities|Map|Remove (Variables|Default|GettileMap) (Variables|Default|GetIndex)))
      (:Is%20Not%20Valid
        (Development|PrintString "Tile not vaild")))))

(fn RepositionPawns
  (for _index (range 0 (- (Utilities|Map|Length (Variables|Default|GettileMap)) 1))
    (Variables|Default|SetIndex _index)
    (Utilities|IsValid (.occupiedpawn (.Value (Utilities|Map|Find (Variables|Default|GettileMap) (Variables|Default|GetIndex))))
      (:Is%20Valid
        (Transformation|SetActorLocation (.occupiedpawn (.Value (Utilities|Map|Find (Variables|Default|GettileMap) (Variables|Default|GetIndex)))) (Transformation|GetWorldLocation (.tilecomponentref (.Value (Utilities|Map|Find (Variables|Default|GettileMap) (Variables|Default|GetIndex))))) false false)))))