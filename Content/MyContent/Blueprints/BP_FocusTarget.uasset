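; BP_FocusTarget is an actor that oscillates back and forth along a configurable axis around its spawn location.
; BeginPlay stores the start location, and Tick calls PingPong to move the actor by frame delta time, speed, multiplier and direction.
; Once it reaches Distance from the start, it snaps to that limit and flips direction, using non-swept moves.
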(event EventBeginPlay
  (Variables|Default|SetstartLocation (Transformation|GetActorLocation)))

(event EventTick
  (params (DeltaSeconds :type Float%20%28single-precision%29))
  (CallFunction|PingPong))

(fn ConstructionScript)

(fn PingPong
  (Transformation|SetActorLocation (+ (* (Utilities|Time|GetWorldDeltaSeconds) (* (Variables|Default|Getspeed) (Variables|Default|GetspeedMultiplier)) (Variables|Default|Getdirection) (Variables|Default|Getaxis)) (Transformation|GetActorLocation)) false false)
  (if (>= (Math|Vector|VectorLength (- (Transformation|GetActorLocation) (Variables|Default|GetstartLocation))) (Variables|Default|Getdistance))
    (Transformation|SetActorLocation (+ (Variables|Default|GetstartLocation) (* (Variables|Default|Getaxis) (Variables|Default|Getdistance) (Variables|Default|Getdirection))) false false)
    (Variables|Default|Setdirection (* (Variables|Default|Getdirection) -1.0))))