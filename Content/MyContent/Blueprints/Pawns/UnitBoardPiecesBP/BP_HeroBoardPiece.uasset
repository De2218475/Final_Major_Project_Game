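; Hero piece on the tile board of a card game, filled from its DT_HeroCardLibrary row in the construction script.
; On click, if match and player states allow, it picks one of five sequenced actions using the LevelManager's ActionTimeline.
; Move looks up the target through the board's direction and tile maps and relocates onto active, free tiles without updating TilePosition.
; Attack is an empty stub, and the direction-widget code is unconnected.
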(event EventBeginPlay
  (|CallParentFunction))

(event Collision|EventActorBeginOverlap
  (params (OtherActor :type Actor%20Object%20Reference))
  (|CallParentFunction OtherActor) ; This node is disabled and will not be called.\nDrag off pins to build functionality.
)

(event EventTick
  (params (DeltaSeconds :type Float%20%28single-precision%29))
  (|CallParentFunction DeltaSeconds) ; This node is disabled and will not be called.\nDrag off pins to build functionality.
)

(event MouseInput|EventActorOnClicked
  (params (ButtonPressed :type Key%20Structure :default "None"))
  (bind _asbp_tcgplayer (Utilities|Casting|CastToBP_TCGPlayer (Game|Player|GetPlayerPawn 0)))
  (bind _output_get (Variables|Default|SetAs%20BP%20TCGPlayer _asbp_tcgplayer))
  (bind _returnvalue (Actor|GetActorOfClass "/Game/MyContent/Blueprints/Gamemodes/TCGGamemode/SinglePlayer/GamemodeElements/LevelManager/LevelManager.LevelManager_C"))
  (bind _output_get_2 (Variables|Default|SetLevelManager _returnvalue))
  (if (and (Utilities|Enum|Equal(Enum) (Variables|/Game/MyContent/Blueprints/Gamemodes/TCGGamemode/SinglePlayer/GamemodeElements/LevelManager/LevelManager.LevelManager_C|GetMatchStates _output_get_2) "NewEnumerator3") (Utilities|Enum|Equal(Enum) (Variables|/Game/MyContent/Blueprints/Gamemodes/TCGGamemode/SinglePlayer/BP_TCGPlayer.BP_TCGPlayer_C|GetCurrentPlayerState _output_get) "NewEnumerator6"))
    (CallFunction|ExecuteAction)))

(event EventExecuteAction
  (bind _heropawndata (Variables|Default|GetHeroPawnData))
  (switch Utilities|FlowControl|Switch|SwitchonE_ActionTimeline (Variables|/Game/MyContent/Blueprints/Gamemodes/TCGGamemode/SinglePlayer/GamemodeElements/LevelManager/LevelManager.LevelManager_C|GetActionTimeline (Variables|Default|GetLevelManager))
    (:NewEnumerator0
      (Variables|Default|SetActionToPerform (.action_1 (.pawnactionseqence _heropawndata))))
    (:NewEnumerator1
      (Variables|Default|SetActionToPerform (.action_2 (.pawnactionseqence _heropawndata))))
    (:NewEnumerator2
      (Variables|Default|SetActionToPerform (.action_3 (.pawnactionseqence _heropawndata))))
    (:NewEnumerator3
      (Variables|Default|SetActionToPerform (.action_4 (.pawnactionseqence _heropawndata))))
    (:NewEnumerator4
      (Variables|Default|SetActionToPerform (.action_5 (.pawnactionseqence _heropawndata)))))
  (CallFunction|PerformAction (.actiontype (Variables|Default|GetActionToPerform))))

(fn ConstructionScript
  (bind _basepiecedata (Variables|Default|GetBasePieceData))
  (|CallParentFunction)
  (bind _returnvalue (Utilities|GetDataTableRow "/Game/MyContent/Blueprints/Cards/CardData/DataTables/HeroCardDTs/DT_HeroCardLibrary.DT_HeroCardLibrary" (.parentcard (Variables|Default|GetBasePieceData)))
    (:then
      (Variables|Default|SetHeroPawnData (Utilities|Struct|MakeStr_HeroPawnDataStructure (.parentcard _basepiecedata) (.tileposition _basepiecedata) (.characterhealthpoints _returnvalue) (.characterattackpoints _returnvalue) (.characterspeedpoints _returnvalue) (.characteractionsequence _returnvalue))))))

(fn PerformAction
  (params (ActionTypeInput :type String))
  (bind _actiontoperform (Variables|Default|GetActionToPerform))
  (bind _actiontoperform_2 (Variables|Default|GetActionToPerform))
  (if (Utilities|Enum|Equal(Enum) ActionTypeInput "Move")
    (CallFunction|Move (.actiondirection _actiontoperform_2) (.actiondistance _actiontoperform_2))
    (elif (Utilities|Enum|Equal(Enum) ActionTypeInput "Attack")
      (CallFunction|Attack (.actiondirection _actiontoperform) (.actiondistance _actiontoperform))
      (else
        (Development|PrintString "InvalidActionType")))))

(fn Move
  (params (ActionDirectionInput :type String) (ActionDistanceInput :type String))
  (bind _heropawndata (Variables|Default|GetHeroPawnData))
  (bind _chessboardref (Variables|Default|GetChessBoardRef))
  (bind _chessboardref_2 (Variables|Default|GetChessBoardRef))
  (bind _tilemap (Variables|/Game/MyContent/Blueprints/Board/BP_ChessBoard.BP_ChessBoard_C|GettileMap _chessboardref))
  (bind _actiondirectionmap (Variables|/Game/MyContent/Blueprints/Board/BP_ChessBoard.BP_ChessBoard_C|GetActionDirectionMap _chessboardref_2))
  (bind _value (Utilities|Map|Find _actiondirectionmap ActionDirectionInput))
  (bind _returnvalue (+ _value (.tileposition _heropawndata)))
  (bind _returnvalue_2 (* _returnvalue ActionDistanceInput))
  (bind _value_2 (Utilities|Map|Find _tilemap _returnvalue_2))
  (if (and (.istileactive _value_2) (.istilefree _value_2))
    (Transformation|SetActorLocation (+ (Transformation|GetWorldLocation (.tilecomponentref _value_2)) "0.000000,0.000000,0.100000") false false)))

(fn Attack
  (params (ActionDirectionInput :type String) (ActionDistanceInput :type String)))