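; Base board piece pawn for a TCG board game, with empty ExecuteAction and OnDamagedCheck events.
; Construction rotates it by facing direction and scales its icon and priority text to the chessboard's tile size.
; Clicks check match state, player state and owning character, then either open a pawn-direction widget or assign the piece to the selected priority slot.
; Priority assignment clears the piece from other slots and updates its number label.
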(event Custom|ExecuteAction)

(event Custom|OnDamagedCheck)

(event EventBeginPlay
  (bind _asbp_tcgplayer (Utilities|Casting|CastToBP_TCGPlayer (Game|Player|GetPlayerPawn 0)))
  (Variables|Default|SetAs%20BP%20TCGPlayer _asbp_tcgplayer)
  (bind _returnvalue (Actor|GetActorOfClass "/Game/MyContent/Blueprints/Gamemodes/TCGGamemode/SinglePlayer/GamemodeElements/LevelManager/LevelManager.LevelManager_C"))
  (Utilities|IsValid _returnvalue
    (:Is%20Valid
      (Variables|Default|SetLevelManager _returnvalue))))

(event MouseInput|EventActorOnClicked
  (params (ButtonPressed :type Key%20Structure :default "None"))
  (for _array_element (Variables|/Game/MyContent/Blueprints/Gamemodes/TCGGamemode/SinglePlayer/GamemodeElements/LevelManager/LevelManager.LevelManager_C|GetCharacterList (Variables|Default|GetLevelManager))
    (bind _asbp_tcgplayer (Utilities|Casting|CastToBP_TCGPlayer (.characterreference _array_element)))
    (Variables|Default|SetAs%20BP%20TCGPlayer _asbp_tcgplayer)
    (if (.ReturnValue (Game|Player|GetHitResultUnderCursorbyChannel (Game|GetPlayerController (.playerindex _array_element)) "TraceTypeQuery1" true))
      (if (Math|Boolean|ANDBoolean (Utilities|Enum|Equal(Enum) (Variables|/Game/MyContent/Blueprints/Gamemodes/TCGGamemode/SinglePlayer/GamemodeElements/LevelManager/LevelManager.LevelManager_C|GetMatchStates (Variables|Default|GetLevelManager)) "NewEnumerator3") (Utilities|Enum|Equal(Enum) (Variables|/Game/MyContent/Blueprints/Gamemodes/TCGGamemode/SinglePlayer/PlayerRelated/BP_TCGPlayer.BP_TCGPlayer_C|GetCurrentPlayerState (Variables|Default|GetAs%20BP%20TCGPlayer)) "NewEnumerator6") (== (.characterid (.owningcharacter (Variables|Default|GetBasePieceData))) (.characterid (Variables|/Game/MyContent/Blueprints/Gamemodes/TCGGamemode/SinglePlayer/PlayerRelated/BP_TCGPlayer.BP_TCGPlayer_C|GetPlayerInfo (Variables|Default|GetAs%20BP%20TCGPlayer)))))
        (Variables|/Game/MyContent/Blueprints/Gamemodes/TCGGamemode/SinglePlayer/PlayerRelated/BP_TCGPlayer.BP_TCGPlayer_C|SetCurrentPlayerState (Variables|Default|GetAs%20BP%20TCGPlayer) "NewEnumerator7")
        (bind _foundwidgets (Widget|GetAllWidgetsOfClass "/Game/MyContent/Blueprints/Pawns/Widgets/WB_PawnDirection.WB_PawnDirection_C" false))
        (for _array_element_2 _foundwidgets
          (Utilities|IsValid _array_element_2
            (:Is%20Valid
              (Widget|RemovefromParent _array_element_2))))
        (bind _returnvalue (UserInterface|CreateWidget "/Game/MyContent/Blueprints/Pawns/Widgets/WB_PawnDirection.WB_PawnDirection_C" 0 self))
        (bind _output_get (Variables|Default|SetPawnDirectionWidget _returnvalue))
        (UserInterface|Viewport|AddtoViewport _output_get 0)
        (elif (Math|Boolean|ANDBoolean (Utilities|Enum|Equal(Enum) (Variables|/Game/MyContent/Blueprints/Gamemodes/TCGGamemode/SinglePlayer/GamemodeElements/LevelManager/LevelManager.LevelManager_C|GetMatchStates (Variables|Default|GetLevelManager)) "NewEnumerator3") (Utilities|Enum|Equal(Enum) (Variables|/Game/MyContent/Blueprints/Gamemodes/TCGGamemode/SinglePlayer/PlayerRelated/BP_TCGPlayer.BP_TCGPlayer_C|GetCurrentPlayerState (Variables|Default|GetAs%20BP%20TCGPlayer)) "NewEnumerator8") (== (.characterid (.owningcharacter (Variables|Default|GetBasePieceData))) (.characterid (Variables|/Game/MyContent/Blueprints/Gamemodes/TCGGamemode/SinglePlayer/PlayerRelated/BP_TCGPlayer.BP_TCGPlayer_C|GetPlayerInfo (Variables|Default|GetAs%20BP%20TCGPlayer)))))
          (bind _foundwidgets_2 (Widget|GetAllWidgetsOfClass "/Game/MyContent/Blueprints/UserInterface/WB_BoardManagement.WB_BoardManagement_C" true))
          (for _array_element_3 _foundwidgets_2
            (Utilities|IsValid _array_element_3
              (:Is%20Valid
                (Variables|Default|SetBoardManagementWidgetref _array_element_3)
                (bind _foundwidgets_3 (Widget|GetAllWidgetsOfClass "/Game/MyContent/Blueprints/UserInterface/WB_PawnPriority.WB_PawnPriority_C" false))
                (for _array_element_4 _foundwidgets_3
                  (Utilities|IsValid _array_element_4
                    (:Is%20Valid
                      (if (== (Variables|/Game/MyContent/Blueprints/UserInterface/WB_PawnPriority.WB_PawnPriority_C|GetSelectedPawn _array_element_4) self)
                        (Variables|/Game/MyContent/Blueprints/UserInterface/WB_PawnPriority.WB_PawnPriority_C|SetSelectedPawn _array_element_4 0)
                        (Variables|/Game/MyContent/Blueprints/UserInterface/WB_PawnPriority.WB_PawnPriority_C|SetPawnImageTexture2D _array_element_4 0)))))
                (Variables|/Game/MyContent/Blueprints/UserInterface/WB_PawnPriority.WB_PawnPriority_C|SetSelectedPawn (Variables|/Game/MyContent/Blueprints/UserInterface/WB_BoardManagement.WB_BoardManagement_C|GetSelectedPawnPriorityWidget (Variables|Default|GetBoardManagementWidgetref)) self)
                (Variables|/Game/MyContent/Blueprints/UserInterface/WB_PawnPriority.WB_PawnPriority_C|SetPawnImageTexture2D (Variables|/Game/MyContent/Blueprints/UserInterface/WB_BoardManagement.WB_BoardManagement_C|GetSelectedPawnPriorityWidget (Variables|Default|GetBoardManagementWidgetref)) (Variables|Default|GetPawnImageTexture2D))
                (Rendering|Components|TextRender|SetText (Variables|Default|GetPriorityNumber) (Variables|/Script/UMG.TextBlock|GetText (Variables|/Game/MyContent/Blueprints/UserInterface/WB_PawnPriority.WB_PawnPriority_C|GetPriorityNumberText (Variables|/Game/MyContent/Blueprints/UserInterface/WB_BoardManagement.WB_BoardManagement_C|GetSelectedPawnPriorityWidget (Variables|Default|GetBoardManagementWidgetref)))))
                (bind _outactors (Actor|GetAllActorsOfClass "BP_BoardPieceBase_C"))
                (for _array_element_5 _outactors
                  (Rendering|Material|SetMaterial (Variables|BP_BoardPieceBase_C|GetBoardPieceIcon _array_element_5) 0 0)
                  (bind _foundwidgets_4 (Widget|GetAllWidgetsOfClass "/Game/MyContent/Blueprints/UserInterface/WB_PawnPriority.WB_PawnPriority_C" false))
                  (for _array_element_6 _foundwidgets_4
                    (Variables|/Game/MyContent/Blueprints/UserInterface/WB_PawnPriority.WB_PawnPriority_C|SetisSelecting? _array_element_6 false))
                  (Variables|/Game/MyContent/Blueprints/Gamemodes/TCGGamemode/SinglePlayer/PlayerRelated/BP_TCGPlayer.BP_TCGPlayer_C|SetCurrentPlayerState (Variables|Default|GetAs%20BP%20TCGPlayer) "NewEnumerator6"))))))))))

(fn ConstructionScript
  (Transformation|SetActorRotation (.Value (Utilities|Map|Find (Variables|Default|GetFaceDirections) (.pawnfacedirection (Variables|Default|GetBasePieceData)))))
  (bind _returnvalue (Actor|GetActorOfClass "/Game/MyContent/Blueprints/Board/BP_ChessBoard.BP_ChessBoard_C"))
  (bind _output_get (Variables|Default|SetChessBoardRef _returnvalue))
  (Utilities|IsValid _output_get
    (:Is%20Valid
      (Transformation|SetWorldScale3D (Variables|Default|GetBoardPieceIcon) (Math|Conversions|ToVector(Float) (/ (Variables|/Game/MyContent/Blueprints/Board/BP_ChessBoard.BP_ChessBoard_C|GettileSize (Variables|Default|GetChessBoardRef)) 8e+02)))
      (Rendering|Components|TextRender|SetWorldSize (Variables|Default|GetPriorityNumber) (* (Variables|/Game/MyContent/Blueprints/Board/BP_ChessBoard.BP_ChessBoard_C|GettileSize (Variables|Default|GetChessBoardRef)) 2e+01)))
    (:Is%20Not%20Valid
      (Development|PrintString "Chess Board Invalid"))))