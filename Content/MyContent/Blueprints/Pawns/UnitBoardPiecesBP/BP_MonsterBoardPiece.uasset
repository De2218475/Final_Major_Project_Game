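; Monster board piece that loads stats and a five-step action sequence from its card's data table row and shows a pawn sprite by team.
; ExecuteAction picks the step matching the LevelManager timeline and PerformAction routes it to Move or Attack.
; Both remap directions by facing to find the target tile; Attack subtracts attack points from hero or monster occupants.
; OnDamagedCheck spawns an explosion and, at zero health, notifies LevelManager and destroys the piece.
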(event EventBeginPlay
  (bind _basepiecedata (Variables|Default|GetBasePieceData))
  (|CallParentFunction)
  (if (== (.teamid (.owningcharacter _basepiecedata)) 0)
    (Rendering|Components|Sprite|SetSprite (Variables|Default|GetBoardPieceIcon) "/Game/ChessSprites/Sprites/b_pawn_png_512px_Sprite.b_pawn_png_512px_Sprite")
    (Variables|Default|SetPawnImageTexture2D "/Game/ChessSprites/Textures/b_pawn_png_512px.b_pawn_png_512px")
    (elif (== (.teamid (.owningcharacter _basepiecedata)) 1)
      (Rendering|Components|Sprite|SetSprite (Variables|Default|GetBoardPieceIcon) "/Game/ChessSprites/Sprites/w_pawn_png_512px_Sprite.w_pawn_png_512px_Sprite")
      (Variables|Default|SetPawnImageTexture2D "/Game/ChessSprites/Textures/w_pawn_png_512px.w_pawn_png_512px")
      (else
        (Development|PrintString "Invalid Team")))))

(event Collision|EventActorBeginOverlap
  (params (OtherActor :type Actor%20Object%20Reference))
  (|CallParentFunction OtherActor) ; This node is disabled and will not be called.\nDrag off pins to build functionality.
)

(event EventTick
  (params (DeltaSeconds :type Float%20%28single-precision%29))
  (|CallParentFunction DeltaSeconds) ; This node is disabled and will not be called.\nDrag off pins to build functionality.
)

(event MouseInput|EventActorOnClicked
  (params (ButtonPressed :type Key%20Structure :default "None"))
  (|CallParentFunction ButtonPressed))

(event EventExecuteAction
  (bind _monsterpawndata (Variables|Default|GetMonsterPawnData))
  (switch Utilities|FlowControl|Switch|SwitchonE_ActionTimeline (Variables|/Game/MyContent/Blueprints/Gamemodes/TCGGamemode/SinglePlayer/GamemodeElements/LevelManager/LevelManager.LevelManager_C|GetActionTimeline (Variables|Default|GetLevelManager))
    (:NewEnumerator0
      (Variables|Default|SetActionToPerform (.action_1 (.pawnactionsequence _monsterpawndata))))
    (:NewEnumerator1
      (Variables|Default|SetActionToPerform (.action_2 (.pawnactionsequence _monsterpawndata))))
    (:NewEnumerator2
      (Variables|Default|SetActionToPerform (.action_3 (.pawnactionsequence _monsterpawndata))))
    (:NewEnumerator3
      (Variables|Default|SetActionToPerform (.action_4 (.pawnactionsequence _monsterpawndata))))
    (:NewEnumerator4
      (Variables|Default|SetActionToPerform (.action_5 (.pawnactionsequence _monsterpawndata)))))
  (CallFunction|PerformAction (.actiontype (Variables|Default|GetActionToPerform))))

(event EventOnDamagedCheck
  (bind _returnvalue (Transformation|GetActorTransform))
  (bind _levelmanager (Variables|Default|GetLevelManager))
  (Effects|SpawnEmitteratLocation "/Game/StarterContent/Particles/P_Explosion.P_Explosion" (.location _returnvalue) (.rotation _returnvalue) "0.050000,0.050000,0.050000")
  (if (<= (.pawnhealthpoints (Variables|Default|GetMonsterPawnData)) 0)
    (Rendering|SetActorHiddenInGame true)
    (Utilities|IsValid _levelmanager
      (:Is%20Valid
        (Default|OnBoardPieceDied _levelmanager))
      (:Is%20Not%20Valid
        _))
    (Actor|DestroyActor)))

(fn ConstructionScript
  (bind _basepiecedata (Variables|Default|GetBasePieceData))
  (|CallParentFunction)
  (bind _returnvalue (Utilities|GetDataTableRow "/Game/MyContent/Blueprints/Cards/CardData/DataTables/MonsterCardDTs/DT_MonsterCardLibrary.DT_MonsterCardLibrary" (.parentcard (Variables|Default|GetBasePieceData)))
    (:then
      (Variables|Default|SetMonsterPawnData (Utilities|Struct|MakeStr_MonsterPawnDataStructure (.owningcharacter _basepiecedata) (.parentcard _basepiecedata) (.tileposition _basepiecedata) (.pawnfacedirection _basepiecedata) (.characterhealthpoints _returnvalue) (.characterattackpoints _returnvalue) (.characterspeedpoints _returnvalue) (.characteractionsequence _returnvalue)))
      (Variables|Default|SetPawnImageTexture2D 0))))

(fn Move
  (params (ActionDirectionInput :type String) (ActionDistanceInput :type String))
  (LocalVariables|SetActionDirection ActionDirectionInput)
  (LocalVariables|SetActionDistance ActionDistanceInput)
  (if (Math|Boolean|ANDBoolean (.istileactive (.Value (Utilities|Map|Find (Variables|/Game/MyContent/Blueprints/Board/BP_ChessBoard.BP_ChessBoard_C|GettileMap (Variables|Default|GetChessBoardRef)) (* (+ (.Value (Utilities|Map|Find (Variables|/Game/MyContent/Blueprints/Board/BP_ChessBoard.BP_ChessBoard_C|GetActionDirectionMap (Variables|Default|GetChessBoardRef)) (.Value (Utilities|Map|Find (Utilities|Map|MakeMap "F" (.f (.Value (Utilities|Map|Find (Variables|Default|GetActionDirectionOffsetMap) (.pawnfacedirection (Variables|Default|GetMonsterPawnData))))) "B" (.b (.Value (Utilities|Map|Find (Variables|Default|GetActionDirectionOffsetMap) (.pawnfacedirection (Variables|Default|GetMonsterPawnData))))) "L" (.l (.Value (Utilities|Map|Find (Variables|Default|GetActionDirectionOffsetMap) (.pawnfacedirection (Variables|Default|GetMonsterPawnData))))) "R" (.r (.Value (Utilities|Map|Find (Variables|Default|GetActionDirectionOffsetMap) (.pawnfacedirection (Variables|Default|GetMonsterPawnData))))) "LF" (.fl (.Value (Utilities|Map|Find (Variables|Default|GetActionDirectionOffsetMap) (.pawnfacedirection (Variables|Default|GetMonsterPawnData))))) "LB" (.fr (.Value (Utilities|Map|Find (Variables|Default|GetActionDirectionOffsetMap) (.pawnfacedirection (Variables|Default|GetMonsterPawnData))))) "RL" (.bl (.Value (Utilities|Map|Find (Variables|Default|GetActionDirectionOffsetMap) (.pawnfacedirection (Variables|Default|GetMonsterPawnData))))) "RB" (.br (.Value (Utilities|Map|Find (Variables|Default|GetActionDirectionOffsetMap) (.pawnfacedirection (Variables|Default|GetMonsterPawnData)))))) (LocalVariables|GetActionDirection))))) (.tileposition (Variables|Default|GetMonsterPawnData))) (LocalVariables|GetActionDistance))))) (.istilefree (.Value (Utilities|Map|Find (Variables|/Game/MyContent/Blueprints/Board/BP_ChessBoard.BP_ChessBoard_C|GettileMap (Variables|Default|GetChessBoardRef)) (* (+ (.Value (Utilities|Map|Find (Variables|/Game/MyContent/Blueprints/Board/BP_ChessBoard.BP_ChessBoard_C|GetActionDirectionMap (Variables|Default|GetChessBoardRef)) (.Value (Utilities|Map|Find (Utilities|Map|MakeMap "F" (.f (.Value (Utilities|Map|Find (Variables|Default|GetActionDirectionOffsetMap) (.pawnfacedirection (Variables|Default|GetMonsterPawnData))))) "B" (.b (.Value (Utilities|Map|Find (Variables|Default|GetActionDirectionOffsetMap) (.pawnfacedirection (Variables|Default|GetMonsterPawnData))))) "L" (.l (.Value (Utilities|Map|Find (Variables|Default|GetActionDirectionOffsetMap) (.pawnfacedirection (Variables|Default|GetMonsterPawnData))))) "R" (.r (.Value (Utilities|Map|Find (Variables|Default|GetActionDirectionOffsetMap) (.pawnfacedirection (Variables|Default|GetMonsterPawnData))))) "LF" (.fl (.Value (Utilities|Map|Find (Variables|Default|GetActionDirectionOffsetMap) (.pawnfacedirection (Variables|Default|GetMonsterPawnData))))) "LB" (.fr (.Value (Utilities|Map|Find (Variables|Default|GetActionDirectionOffsetMap) (.pawnfacedirection (Variables|Default|GetMonsterPawnData))))) "RL" (.bl (.Value (Utilities|Map|Find (Variables|Default|GetActionDirectionOffsetMap) (.pawnfacedirection (Variables|Default|GetMonsterPawnData))))) "RB" (.br (.Value (Utilities|Map|Find (Variables|Default|GetActionDirectionOffsetMap) (.pawnfacedirection (Variables|Default|GetMonsterPawnData)))))) (LocalVariables|GetActionDirection))))) (.tileposition (Variables|Default|GetMonsterPawnData))) (LocalVariables|GetActionDistance))))) (.ReturnValue (Utilities|Map|Find (Variables|/Game/MyContent/Blueprints/Board/BP_ChessBoard.BP_ChessBoard_C|GettileMap (Variables|Default|GetChessBoardRef)) (* (+ (.Value (Utilities|Map|Find (Variables|/Game/MyContent/Blueprints/Board/BP_ChessBoard.BP_ChessBoard_C|GetActionDirectionMap (Variables|Default|GetChessBoardRef)) (.Value (Utilities|Map|Find (Utilities|Map|MakeMap "F" (.f (.Value (Utilities|Map|Find (Variables|Default|GetActionDirectionOffsetMap) (.pawnfacedirection (Variables|Default|GetMonsterPawnData))))) "B" (.b (.Value (Utilities|Map|Find (Variables|Default|GetActionDirectionOffsetMap) (.pawnfacedirection (Variables|Default|GetMonsterPawnData))))) "L" (.l (.Value (Utilities|Map|Find (Variables|Default|GetActionDirectionOffsetMap) (.pawnfacedirection (Variables|Default|GetMonsterPawnData))))) "R" (.r (.Value (Utilities|Map|Find (Variables|Default|GetActionDirectionOffsetMap) (.pawnfacedirection (Variables|Default|GetMonsterPawnData))))) "LF" (.fl (.Value (Utilities|Map|Find (Variables|Default|GetActionDirectionOffsetMap) (.pawnfacedirection (Variables|Default|GetMonsterPawnData))))) "LB" (.fr (.Value (Utilities|Map|Find (Variables|Default|GetActionDirectionOffsetMap) (.pawnfacedirection (Variables|Default|GetMonsterPawnData))))) "RL" (.bl (.Value (Utilities|Map|Find (Variables|Default|GetActionDirectionOffsetMap) (.pawnfacedirection (Variables|Default|GetMonsterPawnData))))) "RB" (.br (.Value (Utilities|Map|Find (Variables|Default|GetActionDirectionOffsetMap) (.pawnfacedirection (Variables|Default|GetMonsterPawnData)))))) (LocalVariables|GetActionDirection))))) (.tileposition (Variables|Default|GetMonsterPawnData))) (LocalVariables|GetActionDistance)))))
    (Transformation|SetActorLocation (+ (Transformation|GetWorldLocation (.tilecomponentref (.Value (Utilities|Map|Find (Variables|/Game/MyContent/Blueprints/Board/BP_ChessBoard.BP_ChessBoard_C|GettileMap (Variables|Default|GetChessBoardRef)) (* (+ (.Value (Utilities|Map|Find (Variables|/Game/MyContent/Blueprints/Board/BP_ChessBoard.BP_ChessBoard_C|GetActionDirectionMap (Variables|Default|GetChessBoardRef)) (.Value (Utilities|Map|Find (Utilities|Map|MakeMap "F" (.f (.Value (Utilities|Map|Find (Variables|Default|GetActionDirectionOffsetMap) (.pawnfacedirection (Variables|Default|GetMonsterPawnData))))) "B" (.b (.Value (Utilities|Map|Find (Variables|Default|GetActionDirectionOffsetMap) (.pawnfacedirection (Variables|Default|GetMonsterPawnData))))) "L" (.l (.Value (Utilities|Map|Find (Variables|Default|GetActionDirectionOffsetMap) (.pawnfacedirection (Variables|Default|GetMonsterPawnData))))) "R" (.r (.Value (Utilities|Map|Find (Variables|Default|GetActionDirectionOffsetMap) (.pawnfacedirection (Variables|Default|GetMonsterPawnData))))) "LF" (.fl (.Value (Utilities|Map|Find (Variables|Default|GetActionDirectionOffsetMap) (.pawnfacedirection (Variables|Default|GetMonsterPawnData))))) "LB" (.fr (.Value (Utilities|Map|Find (Variables|Default|GetActionDirectionOffsetMap) (.pawnfacedirection (Variables|Default|GetMonsterPawnData))))) "RL" (.bl (.Value (Utilities|Map|Find (Variables|Default|GetActionDirectionOffsetMap) (.pawnfacedirection (Variables|Default|GetMonsterPawnData))))) "RB" (.br (.Value (Utilities|Map|Find (Variables|Default|GetActionDirectionOffsetMap) (.pawnfacedirection (Variables|Default|GetMonsterPawnData)))))) (LocalVariables|GetActionDirection))))) (.tileposition (Variables|Default|GetMonsterPawnData))) (LocalVariables|GetActionDistance)))))) "0.000000,0.000000,0.100000") false false)
    (bind _output_get (Variables|Default|SetMonsterPawnData (Utilities|Struct|MakeStr_MonsterPawnDataStructure (.owningcharacter (Variables|Default|GetMonsterPawnData)) (.parentcardid (Variables|Default|GetMonsterPawnData)) (+ (.Value (Utilities|Map|Find (Variables|/Game/MyContent/Blueprints/Board/BP_ChessBoard.BP_ChessBoard_C|GetActionDirectionMap (Variables|Default|GetChessBoardRef)) (.Value (Utilities|Map|Find (Utilities|Map|MakeMap "F" (.f (.Value (Utilities|Map|Find (Variables|Default|GetActionDirectionOffsetMap) (.pawnfacedirection (Variables|Default|GetMonsterPawnData))))) "B" (.b (.Value (Utilities|Map|Find (Variables|Default|GetActionDirectionOffsetMap) (.pawnfacedirection (Variables|Default|GetMonsterPawnData))))) "L" (.l (.Value (Utilities|Map|Find (Variables|Default|GetActionDirectionOffsetMap) (.pawnfacedirection (Variables|Default|GetMonsterPawnData))))) "R" (.r (.Value (Utilities|Map|Find (Variables|Default|GetActionDirectionOffsetMap) (.pawnfacedirection (Variables|Default|GetMonsterPawnData))))) "LF" (.fl (.Value (Utilities|Map|Find (Variables|Default|GetActionDirectionOffsetMap) (.pawnfacedirection (Variables|Default|GetMonsterPawnData))))) "LB" (.fr (.Value (Utilities|Map|Find (Variables|Default|GetActionDirectionOffsetMap) (.pawnfacedirection (Variables|Default|GetMonsterPawnData))))) "RL" (.bl (.Value (Utilities|Map|Find (Variables|Default|GetActionDirectionOffsetMap) (.pawnfacedirection (Variables|Default|GetMonsterPawnData))))) "RB" (.br (.Value (Utilities|Map|Find (Variables|Default|GetActionDirectionOffsetMap) (.pawnfacedirection (Variables|Default|GetMonsterPawnData)))))) (LocalVariables|GetActionDirection))))) (.tileposition (Variables|Default|GetMonsterPawnData))) (.pawnfacedirection (Variables|Default|GetMonsterPawnData)) (.pawnhealthpoints (Variables|Default|GetMonsterPawnData)) (.pawnattackpoints (Variables|Default|GetMonsterPawnData)) (.pawnspeedpoints (Variables|Default|GetMonsterPawnData)) (.pawnactionsequence (Variables|Default|GetMonsterPawnData)))))
    (Variables|Default|SetBasePieceData (Utilities|Struct|MakeStr_BasePawnDataStructure (.owningcharacter _output_get) (.parentcardid _output_get) (.tileposition _output_get) (.pawnfacedirection _output_get)))))

(fn Attack
  (params (ActionDirectionInput :type String) (ActionDistanceInput :type String))
  (LocalVariables|SetActionDirection ActionDirectionInput)
  (LocalVariables|SetActionDistance ActionDistanceInput)
  (Development|PrintString "trigger attack")
  (if (and (.istileactive (.Value (Utilities|Map|Find (Variables|/Game/MyContent/Blueprints/Board/BP_ChessBoard.BP_ChessBoard_C|GettileMap (Variables|Default|GetChessBoardRef)) (* (+ (.Value (Utilities|Map|Find (Variables|/Game/MyContent/Blueprints/Board/BP_ChessBoard.BP_ChessBoard_C|GetActionDirectionMap (Variables|Default|GetChessBoardRef)) (.Value (Utilities|Map|Find (Utilities|Map|MakeMap "F" (.f (.Value (Utilities|Map|Find (Variables|Default|GetActionDirectionOffsetMap) (.pawnfacedirection (Variables|Default|GetMonsterPawnData))))) "B" (.b (.Value (Utilities|Map|Find (Variables|Default|GetActionDirectionOffsetMap) (.pawnfacedirection (Variables|Default|GetMonsterPawnData))))) "L" (.l (.Value (Utilities|Map|Find (Variables|Default|GetActionDirectionOffsetMap) (.pawnfacedirection (Variables|Default|GetMonsterPawnData))))) "R" (.r (.Value (Utilities|Map|Find (Variables|Default|GetActionDirectionOffsetMap) (.pawnfacedirection (Variables|Default|GetMonsterPawnData))))) "LF" (.fl (.Value (Utilities|Map|Find (Variables|Default|GetActionDirectionOffsetMap) (.pawnfacedirection (Variables|Default|GetMonsterPawnData))))) "LB" (.fr (.Value (Utilities|Map|Find (Variables|Default|GetActionDirectionOffsetMap) (.pawnfacedirection (Variables|Default|GetMonsterPawnData))))) "RL" (.bl (.Value (Utilities|Map|Find (Variables|Default|GetActionDirectionOffsetMap) (.pawnfacedirection (Variables|Default|GetMonsterPawnData))))) "RB" (.br (.Value (Utilities|Map|Find (Variables|Default|GetActionDirectionOffsetMap) (.pawnfacedirection (Variables|Default|GetMonsterPawnData)))))) (LocalVariables|GetActionDirection))))) (.tileposition (Variables|Default|GetMonsterPawnData))) (LocalVariables|GetActionDistance))))) (not (.istilefree (.Value (Utilities|Map|Find (Variables|/Game/MyContent/Blueprints/Board/BP_ChessBoard.BP_ChessBoard_C|GettileMap (Variables|Default|GetChessBoardRef)) (* (+ (.Value (Utilities|Map|Find (Variables|/Game/MyContent/Blueprints/Board/BP_ChessBoard.BP_ChessBoard_C|GetActionDirectionMap (Variables|Default|GetChessBoardRef)) (.Value (Utilities|Map|Find (Utilities|Map|MakeMap "F" (.f (.Value (Utilities|Map|Find (Variables|Default|GetActionDirectionOffsetMap) (.pawnfacedirection (Variables|Default|GetMonsterPawnData))))) "B" (.b (.Value (Utilities|Map|Find (Variables|Default|GetActionDirectionOffsetMap) (.pawnfacedirection (Variables|Default|GetMonsterPawnData))))) "L" (.l (.Value (Utilities|Map|Find (Variables|Default|GetActionDirectionOffsetMap) (.pawnfacedirection (Variables|Default|GetMonsterPawnData))))) "R" (.r (.Value (Utilities|Map|Find (Variables|Default|GetActionDirectionOffsetMap) (.pawnfacedirection (Variables|Default|GetMonsterPawnData))))) "LF" (.fl (.Value (Utilities|Map|Find (Variables|Default|GetActionDirectionOffsetMap) (.pawnfacedirection (Variables|Default|GetMonsterPawnData))))) "LB" (.fr (.Value (Utilities|Map|Find (Variables|Default|GetActionDirectionOffsetMap) (.pawnfacedirection (Variables|Default|GetMonsterPawnData))))) "RL" (.bl (.Value (Utilities|Map|Find (Variables|Default|GetActionDirectionOffsetMap) (.pawnfacedirection (Variables|Default|GetMonsterPawnData))))) "RB" (.br (.Value (Utilities|Map|Find (Variables|Default|GetActionDirectionOffsetMap) (.pawnfacedirection (Variables|Default|GetMonsterPawnData)))))) (LocalVariables|GetActionDirection))))) (.tileposition (Variables|Default|GetMonsterPawnData))) (LocalVariables|GetActionDistance)))))))
    (Utilities|IsValid (.occupiedpawn (.Value (Utilities|Map|Find (Variables|/Game/MyContent/Blueprints/Board/BP_ChessBoard.BP_ChessBoard_C|GettileMap (Variables|Default|GetChessBoardRef)) (* (+ (.Value (Utilities|Map|Find (Variables|/Game/MyContent/Blueprints/Board/BP_ChessBoard.BP_ChessBoard_C|GetActionDirectionMap (Variables|Default|GetChessBoardRef)) (.Value (Utilities|Map|Find (Utilities|Map|MakeMap "F" (.f (.Value (Utilities|Map|Find (Variables|Default|GetActionDirectionOffsetMap) (.pawnfacedirection (Variables|Default|GetMonsterPawnData))))) "B" (.b (.Value (Utilities|Map|Find (Variables|Default|GetActionDirectionOffsetMap) (.pawnfacedirection (Variables|Default|GetMonsterPawnData))))) "L" (.l (.Value (Utilities|Map|Find (Variables|Default|GetActionDirectionOffsetMap) (.pawnfacedirection (Variables|Default|GetMonsterPawnData))))) "R" (.r (.Value (Utilities|Map|Find (Variables|Default|GetActionDirectionOffsetMap) (.pawnfacedirection (Variables|Default|GetMonsterPawnData))))) "LF" (.fl (.Value (Utilities|Map|Find (Variables|Default|GetActionDirectionOffsetMap) (.pawnfacedirection (Variables|Default|GetMonsterPawnData))))) "LB" (.fr (.Value (Utilities|Map|Find (Variables|Default|GetActionDirectionOffsetMap) (.pawnfacedirection (Variables|Default|GetMonsterPawnData))))) "RL" (.bl (.Value (Utilities|Map|Find (Variables|Default|GetActionDirectionOffsetMap) (.pawnfacedirection (Variables|Default|GetMonsterPawnData))))) "RB" (.br (.Value (Utilities|Map|Find (Variables|Default|GetActionDirectionOffsetMap) (.pawnfacedirection (Variables|Default|GetMonsterPawnData)))))) (LocalVariables|GetActionDirection))))) (.tileposition (Variables|Default|GetMonsterPawnData))) (LocalVariables|GetActionDistance)))))
      (:Is%20Valid
        (bind _asbp_hero_board_piece (Utilities|Casting|CastToBP_HeroBoardPiece (.occupiedpawn (.Value (Utilities|Map|Find (Variables|/Game/MyContent/Blueprints/Board/BP_ChessBoard.BP_ChessBoard_C|GettileMap (Variables|Default|GetChessBoardRef)) (* (+ (.Value (Utilities|Map|Find (Variables|/Game/MyContent/Blueprints/Board/BP_ChessBoard.BP_ChessBoard_C|GetActionDirectionMap (Variables|Default|GetChessBoardRef)) (.Value (Utilities|Map|Find (Utilities|Map|MakeMap "F" (.f (.Value (Utilities|Map|Find (Variables|Default|GetActionDirectionOffsetMap) (.pawnfacedirection (Variables|Default|GetMonsterPawnData))))) "B" (.b (.Value (Utilities|Map|Find (Variables|Default|GetActionDirectionOffsetMap) (.pawnfacedirection (Variables|Default|GetMonsterPawnData))))) "L" (.l (.Value (Utilities|Map|Find (Variables|Default|GetActionDirectionOffsetMap) (.pawnfacedirection (Variables|Default|GetMonsterPawnData))))) "R" (.r (.Value (Utilities|Map|Find (Variables|Default|GetActionDirectionOffsetMap) (.pawnfacedirection (Variables|Default|GetMonsterPawnData))))) "LF" (.fl (.Value (Utilities|Map|Find (Variables|Default|GetActionDirectionOffsetMap) (.pawnfacedirection (Variables|Default|GetMonsterPawnData))))) "LB" (.fr (.Value (Utilities|Map|Find (Variables|Default|GetActionDirectionOffsetMap) (.pawnfacedirection (Variables|Default|GetMonsterPawnData))))) "RL" (.bl (.Value (Utilities|Map|Find (Variables|Default|GetActionDirectionOffsetMap) (.pawnfacedirection (Variables|Default|GetMonsterPawnData))))) "RB" (.br (.Value (Utilities|Map|Find (Variables|Default|GetActionDirectionOffsetMap) (.pawnfacedirection (Variables|Default|GetMonsterPawnData)))))) (LocalVariables|GetActionDirection))))) (.tileposition (Variables|Default|GetMonsterPawnData))) (LocalVariables|GetActionDistance))))))
          (:then
            (bind _output_get (Variables|Default|SetAs%20BP%20Hero%20Board%20Piece _asbp_hero_board_piece))
            (Variables|/Game/MyContent/Blueprints/Pawns/UnitBoardPiecesBP/BP_HeroBoardPiece.BP_HeroBoardPiece_C|SetHeroPawnData (Variables|Default|GetAs%20BP%20Hero%20Board%20Piece) (Utilities|Struct|MakeStr_HeroPawnDataStructure (.owningcharacter (Variables|/Game/MyContent/Blueprints/Pawns/UnitBoardPiecesBP/BP_HeroBoardPiece.BP_HeroBoardPiece_C|GetHeroPawnData _output_get)) (.parentcardid (Variables|/Game/MyContent/Blueprints/Pawns/UnitBoardPiecesBP/BP_HeroBoardPiece.BP_HeroBoardPiece_C|GetHeroPawnData _output_get)) (.tileposition (Variables|/Game/MyContent/Blueprints/Pawns/UnitBoardPiecesBP/BP_HeroBoardPiece.BP_HeroBoardPiece_C|GetHeroPawnData _output_get)) (.pawnfacedirection (Variables|/Game/MyContent/Blueprints/Pawns/UnitBoardPiecesBP/BP_HeroBoardPiece.BP_HeroBoardPiece_C|GetHeroPawnData _output_get)) (- (.pawnhealthpoints (Variables|/Game/MyContent/Blueprints/Pawns/UnitBoardPiecesBP/BP_HeroBoardPiece.BP_HeroBoardPiece_C|GetHeroPawnData _output_get)) (.pawnattackpoints (Variables|Default|GetMonsterPawnData))) (.pawnattackpoints (Variables|/Game/MyContent/Blueprints/Pawns/UnitBoardPiecesBP/BP_HeroBoardPiece.BP_HeroBoardPiece_C|GetHeroPawnData _output_get)) (.pawnspeedpoints (Variables|/Game/MyContent/Blueprints/Pawns/UnitBoardPiecesBP/BP_HeroBoardPiece.BP_HeroBoardPiece_C|GetHeroPawnData _output_get)) (.pawnactionseqence (Variables|/Game/MyContent/Blueprints/Pawns/UnitBoardPiecesBP/BP_HeroBoardPiece.BP_HeroBoardPiece_C|GetHeroPawnData _output_get))))
            (Default|OnDamagedCheck (Variables|Default|GetAs%20BP%20Hero%20Board%20Piece)))
          (:CastFailed
            (bind _asbp_monster_board_piece (Utilities|Casting|CastToBP_MonsterBoardPiece (.occupiedpawn (.Value (Utilities|Map|Find (Variables|/Game/MyContent/Blueprints/Board/BP_ChessBoard.BP_ChessBoard_C|GettileMap (Variables|Default|GetChessBoardRef)) (* (+ (.Value (Utilities|Map|Find (Variables|/Game/MyContent/Blueprints/Board/BP_ChessBoard.BP_ChessBoard_C|GetActionDirectionMap (Variables|Default|GetChessBoardRef)) (.Value (Utilities|Map|Find (Utilities|Map|MakeMap "F" (.f (.Value (Utilities|Map|Find (Variables|Default|GetActionDirectionOffsetMap) (.pawnfacedirection (Variables|Default|GetMonsterPawnData))))) "B" (.b (.Value (Utilities|Map|Find (Variables|Default|GetActionDirectionOffsetMap) (.pawnfacedirection (Variables|Default|GetMonsterPawnData))))) "L" (.l (.Value (Utilities|Map|Find (Variables|Default|GetActionDirectionOffsetMap) (.pawnfacedirection (Variables|Default|GetMonsterPawnData))))) "R" (.r (.Value (Utilities|Map|Find (Variables|Default|GetActionDirectionOffsetMap) (.pawnfacedirection (Variables|Default|GetMonsterPawnData))))) "LF" (.fl (.Value (Utilities|Map|Find (Variables|Default|GetActionDirectionOffsetMap) (.pawnfacedirection (Variables|Default|GetMonsterPawnData))))) "LB" (.fr (.Value (Utilities|Map|Find (Variables|Default|GetActionDirectionOffsetMap) (.pawnfacedirection (Variables|Default|GetMonsterPawnData))))) "RL" (.bl (.Value (Utilities|Map|Find (Variables|Default|GetActionDirectionOffsetMap) (.pawnfacedirection (Variables|Default|GetMonsterPawnData))))) "RB" (.br (.Value (Utilities|Map|Find (Variables|Default|GetActionDirectionOffsetMap) (.pawnfacedirection (Variables|Default|GetMonsterPawnData)))))) (LocalVariables|GetActionDirection))))) (.tileposition (Variables|Default|GetMonsterPawnData))) (LocalVariables|GetActionDistance))))))
              (:then
                (bind _output_get_2 (Variables|Default|SetAs%20BP%20Monster%20Board%20Piece _asbp_monster_board_piece))
                (Variables|BP_MonsterBoardPiece_C|SetMonsterPawnData (Variables|Default|GetAs%20BP%20Monster%20Board%20Piece) (Utilities|Struct|MakeStr_MonsterPawnDataStructure (.owningcharacter (Variables|BP_MonsterBoardPiece_C|GetMonsterPawnData _output_get_2)) (.parentcardid (Variables|BP_MonsterBoardPiece_C|GetMonsterPawnData _output_get_2)) (.tileposition (Variables|BP_MonsterBoardPiece_C|GetMonsterPawnData _output_get_2)) (.pawnfacedirection (Variables|BP_MonsterBoardPiece_C|GetMonsterPawnData _output_get_2)) (- (.pawnhealthpoints (Variables|BP_MonsterBoardPiece_C|GetMonsterPawnData _output_get_2)) (.pawnattackpoints (Variables|Default|GetMonsterPawnData))) (.pawnattackpoints (Variables|BP_MonsterBoardPiece_C|GetMonsterPawnData _output_get_2)) (.pawnspeedpoints (Variables|BP_MonsterBoardPiece_C|GetMonsterPawnData _output_get_2)) (.pawnactionsequence (Variables|BP_MonsterBoardPiece_C|GetMonsterPawnData _output_get_2))))
                (Default|OnDamagedCheck (Variables|Default|GetAs%20BP%20Monster%20Board%20Piece)))
              (:CastFailed
                (Development|PrintString "cast failed")))))))))

(fn PerformAction
  (params (ActionTypeInput :type String))
  (bind _actiontoperform (Variables|Default|GetActionToPerform))
  (bind _actiontoperform_2 (Variables|Default|GetActionToPerform))
  (if (Utilities|Enum|Equal(Enum) ActionTypeInput "Move")
    (CallFunction|Move (.actiondirection _actiontoperform_2) (.actiondistance _actiontoperform_2))
    (elif (Utilities|Enum|Equal(Enum) ActionTypeInput "Attack")
      (CallFunction|Attack (.actiondirection _actiontoperform) (.actiondistance _actiontoperform))
      (else
        (Development|PrintString "InvalidActionType")))))