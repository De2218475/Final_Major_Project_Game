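; Player for the TCG game mode that manages a camera moving between named preset positions, with mouse cursor and click input enabled.
; Key 1 cycles positions via an index-to-name map built in the construction script; key 2 toggles target focus.
; Tick lerps and snaps the camera transform, moving only location while focused so look-at rotation runs without jitter.
; PlacingPawn highlights free chessboard spawn tiles and switches to the Board view.
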(event Custom|CalcNextCameraPosition
  ;[0 0 0 1 12] Custom event used to update the next camera position to switch to. This gets called when the camera needs to be switched.
  (if (Variables|PlayerCamera|GetCanSwitchCamera)
    (Variables|PlayerCamera|SetCameraInPosition false)
    (if (>= (Variables|PlayerCamera|GetCurrentCamPositionINT) (- (Utilities|Map|Length (Variables|PlayerCamera|GetCameraPositionFinder)) 1))
      (Variables|PlayerCamera|SetCurrentCamPositionINT 0)
      (else
        (Math|Integer|IncrementInt (Variables|PlayerCamera|GetCurrentCamPositionINT)
          (:%20%20
            _))))
    (Variables|PlayerCamera|SetCurrentCameraPosition (.Value (Utilities|Map|Find (Variables|PlayerCamera|GetCameraPositionFinder) (Variables|PlayerCamera|GetCurrentCamPositionINT))))))

(event Custom|SwitchCameraPosition
  (bind _returnvalue (Utilities|Time|GetWorldDeltaSeconds))
  (bind _returnvalue_2 (Utilities|Time|GetWorldDeltaSeconds))
  (bind _playercamera (Variables|Default|GetPlayerCamera))
  (bind _cameratransitionspeed (Variables|PlayerCamera|GetCameraTransitionSpeed))
  (bind _cameratransitionspeed_2 (Variables|PlayerCamera|GetCameraTransitionSpeed))
  (bind _playercamera_2 (Variables|Default|GetPlayerCamera))
  (bind _currentcameraposition (Variables|PlayerCamera|GetCurrentCameraPosition))
  (bind _camerapositions (Variables|PlayerCamera|GetCameraPositions))
  (bind _currentcameraposition_2 (Variables|PlayerCamera|GetCurrentCameraPosition))
  (bind _camerapositions_2 (Variables|PlayerCamera|GetCameraPositions))
  (bind _returnvalue_3 (Transformation|GetWorldLocation _playercamera_2))
  (bind _returnvalue_4 (Transformation|GetWorldTransform _playercamera))
  (bind _value (Utilities|Map|Find _camerapositions _currentcameraposition))
  (bind _value_2 (Utilities|Map|Find _camerapositions_2 _currentcameraposition_2))
  (bind _returnvalue_5 (* _returnvalue _cameratransitionspeed))
  (bind _returnvalue_6 (* _returnvalue_2 _cameratransitionspeed_2))
  (bind _returnvalue_7 (Math|Float|Clamp(Float) _returnvalue_5))
  (bind _returnvalue_8 (Math|Float|Clamp(Float) _returnvalue_6))
  (bind _returnvalue_9 (Math|Vector|Lerp(Vector) _returnvalue_3 (.location _value) _returnvalue_7))
  (bind _returnvalue_10 (Math|Transform|Lerp(Transform) _returnvalue_4 _value_2 _returnvalue_8))
  ;[0 0 0 1 12] Custom event used for switching the camera to the next target position. This event is handled in the Event Tick and is only executed if camera is not in position.
  (if (not (Variables|PlayerCamera|GetCameraInPosition))
    ;[0 0 0 1 12] Once the camera is not in position, a check is made to see if the camera is focusing on an object. If the camera is focused, then its location is changed to match the target camera location. If the camera is not focused, then it will change its entire transform to match the target camera position. This is necessary to avoid clashing camera updates between the focus target and target camera position, which would cause jittering and extra processing.
    (if (Variables|PlayerCamera|GetShouldFocusTarget)
      ;[0 0 0 1 12] An issue with slower camera speeds is that it takes longer to reach the exact target value when incrementing small decimal values, giving the illusion that it gets stuck in the wrong position. To avoid this, we make a tolerance check so that if the current position is close enough to the target location it will snap to the target location. If the current position is not close enough it will continue lerping to its target location.
      (Variables|PlayerCamera|SetTargetTransform (Math|Transform|MakeTransform _returnvalue_9 "0, 0, 0" "1.000000,1.000000,1.000000"))
      (if (Utilities|Operators|EqualEqual _returnvalue_9 (.location _value) 0.01)
        (Transformation|SetWorldLocation (Variables|Default|GetPlayerCamera) (.location (.Value (Utilities|Map|Find (Variables|PlayerCamera|GetCameraPositions) (Variables|PlayerCamera|GetCurrentCameraPosition)))) false false)
        (else
          (Transformation|SetWorldLocation (Variables|Default|GetPlayerCamera) (.location (Variables|PlayerCamera|GetTargetTransform)) false false)))
      ;[0 0 0 1 12] We then make a final check to see if the current camera location matches the target location. If it matches then it will stop updating the camera position and allow the player to switch again, else it will continue updating.
      (if (Utilities|Operators|EqualEqual (Transformation|GetWorldLocation (Variables|Default|GetPlayerCamera)) (.location (.Value (Utilities|Map|Find (Variables|PlayerCamera|GetCameraPositions) (Variables|PlayerCamera|GetCurrentCameraPosition)))) 0.0)
        (Variables|PlayerCamera|SetCanSwitchCamera true)
        (Variables|PlayerCamera|SetCameraInPosition true)
        (else
          (Variables|PlayerCamera|SetCanSwitchCamera false)
          (Variables|PlayerCamera|SetCameraInPosition false)))
      (else
        (Variables|PlayerCamera|SetTargetTransform _returnvalue_10)
        (if (Class|KismetMathLibrary|NearlyEqualTransformTransform _returnvalue_10 _value_2 0.01 0.01 0.01)
          (Transformation|SetWorldTransform (Variables|Default|GetPlayerCamera) (.Value (Utilities|Map|Find (Variables|PlayerCamera|GetCameraPositions) (Variables|PlayerCamera|GetCurrentCameraPosition))) false false)
          (else
            (Transformation|SetWorldTransform (Variables|Default|GetPlayerCamera) (Variables|PlayerCamera|GetTargetTransform) false false)))
        (if (== (Transformation|GetWorldTransform (Variables|Default|GetPlayerCamera)) (.Value (Utilities|Map|Find (Variables|PlayerCamera|GetCameraPositions) (Variables|PlayerCamera|GetCurrentCameraPosition))))
          (Variables|PlayerCamera|SetCanSwitchCamera true)
          (Variables|PlayerCamera|SetCameraInPosition true)
          (else
            (Variables|PlayerCamera|SetCanSwitchCamera false)
            (Variables|PlayerCamera|SetCameraInPosition false)))))))

(event Custom|FocusTarget
  ;[0 0 0 1 12] Custom event used to update the cameras rotation to look and focus on a specific object. As it updates the camera, this event is handled in the event tick.
  (if (Variables|PlayerCamera|GetShouldFocusTarget)
    (Utilities|IsValid (Variables|PlayerCamera|GetFocusTargetRef)
      (:Is%20Valid
        (Transformation|SetWorldRotation (Variables|Default|GetPlayerCamera) (Math|Rotator|Lerp(Rotator) (Transformation|GetWorldRotation (Variables|Default|GetPlayerCamera)) (Math|Rotator|FindLookatRotation (Transformation|GetWorldLocation (Variables|Default|GetPlayerCamera)) (Transformation|GetActorLocation (Variables|PlayerCamera|GetFocusTargetRef))) (Math|Float|Clamp(Float) (* (Utilities|Time|GetWorldDeltaSeconds) (Variables|PlayerCamera|GetCameraFollowSpeed)))) false false)))))

(event Custom|PlacingPawn
  (Variables|Default|SetCurrentPlayerState "NewEnumerator3")
  (bind _returnvalue (Actor|GetActorOfClass "/Game/MyContent/Blueprints/Board/BP_ChessBoard.BP_ChessBoard_C"))
  (bind _output_get (Variables|Default|SetChessBoardRef _returnvalue))
  (Utilities|IsValid _output_get
    (:Is%20Valid
      (for _index (range 0 (- (Utilities|Map|Length (Variables|/Game/MyContent/Blueprints/Board/BP_ChessBoard.BP_ChessBoard_C|GettileMap _output_get)) 1))
        (bind _output_get_2 (Variables|/Game/MyContent/Blueprints/Board/BP_ChessBoard.BP_ChessBoard_C|SetIndex (Variables|Default|GetChessBoardRef) _index))
        (if (and (.istilefree (.Value (Utilities|Map|Find (Variables|/Game/MyContent/Blueprints/Board/BP_ChessBoard.BP_ChessBoard_C|GettileMap (Variables|Default|GetChessBoardRef)) _output_get_2))) (.isspawntile (.Value (Utilities|Map|Find (Variables|/Game/MyContent/Blueprints/Board/BP_ChessBoard.BP_ChessBoard_C|GettileMap (Variables|Default|GetChessBoardRef)) _output_get_2))))
          (Rendering|Material|SetMaterial (.tilecomponentref (.Value (Utilities|Map|Find (Variables|/Game/MyContent/Blueprints/Board/BP_ChessBoard.BP_ChessBoard_C|GettileMap (Variables|Default|GetChessBoardRef)) _output_get_2))) 0 "/Game/MyContent/Materials/OverlayMAT/MAT_ObjectSelection.MAT_ObjectSelection")
          (Variables|PlayerCamera|SetCurrentCameraPosition "Board")
          (Variables|PlayerCamera|SetCameraInPosition false))))))

(event EventBeginPlay
  (bind _returnvalue (Game|GetPlayerController 0))
  (Variables|/Script/Engine.PlayerController|SetbShowMouseCursor _returnvalue true)
  (Variables|/Script/Engine.PlayerController|SetbEnableClickEvents _returnvalue true)
  (Variables|/Script/Engine.PlayerController|SetbEnableMouseOverEvents _returnvalue true)
  (Input|SetInputModeGameandUI _returnvalue 0 "DoNotLock" false false))

(event EventTick
  (params (DeltaSeconds :type Float%20%28single-precision%29))
  (CallFunction|SwitchCameraPosition)
  (CallFunction|FocusTarget))

(event Input|KeyboardEvents|1
  (params (Key :type Key%20Structure :default "None"))
  ;[0 0 0 1 12] Event used for switching camera to next position.
  (:Pressed
    (CallFunction|CalcNextCameraPosition)
    (Variables|PlayerCamera|SetCanSwitchCamera false)))

(event Input|KeyboardEvents|2
  (params (Key :type Key%20Structure :default "None"))
  ;[0 0 0 1 12] Event used for toggling camera focus on a specific object.
  (:Pressed
    (Utilities|FlowControl|FlipFlop
      (:A
        (Variables|PlayerCamera|SetShouldFocusTarget true))
      (:B
        (Variables|PlayerCamera|SetShouldFocusTarget false)
        (Variables|PlayerCamera|SetCameraInPosition false)))))

(fn ConstructionScript
  (bind _keys (Utilities|Map|Keys (Variables|PlayerCamera|GetCameraPositions)))
  (for (_array_element _array_index) _keys
    (Utilities|Map|Add (Variables|PlayerCamera|GetCameraPositionFinder) _array_index _array_element)))