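; Single-player TCG player that enables mouse interaction, shows the resource counter widget and drives the table cameras.
; Each tick either spins a spring-arm camera or lerps the main camera between named transforms, optionally tracking a focus target.
; The construction script indexes position names so key 1 can cycle them, while key 2 toggles focus.
; Pawn placement and management events set player state and switch to the board view, with placement highlighting free spawn tiles.
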(event Custom|CalcNextCameraPosition
  ;[0 0 0 1 12] Custom event used to update the next camera position to switch to. This gets called when the camera needs to be switched.
  (if (Variables|PlayerCamera|GetCanSwitchCamera)
    (Variables|PlayerCamera|SetCameraInPosition false)
    (if (>= (Variables|PlayerCamera|GetCurrentCamPositionINT) (- (Utilities|Map|Length (Variables|PlayerCamera|GetCameraPositionFinder)) 1))
      (Variables|PlayerCamera|SetCurrentCamPositionINT 0)
      (else
        (Math|Integer|IncrementInt (Variables|PlayerCamera|GetCurrentCamPositionINT)
          (:%20%20
            _))))
    (Variables|PlayerCamera|SetCurrentCameraPosition (.Value (Utilities|Map|Find (Variables|PlayerCamera|GetCameraPositionFinder) (Variables|PlayerCamera|GetCurrentCamPositionINT))))))

(event Custom|PlacingPawn
  (Variables|Default|SetCurrentPlayerState "NewEnumerator3")
  (bind _returnvalue (Actor|GetActorOfClass "/Game/MyContent/Blueprints/Board/BP_ChessBoard.BP_ChessBoard_C"))
  (bind _output_get (Variables|Default|SetChessBoardRef _returnvalue))
  (Utilities|IsValid _output_get
    (:Is%20Valid
      (for _index (range 0 (- (Utilities|Map|Length (Variables|/Game/MyContent/Blueprints/Board/BP_ChessBoard.BP_ChessBoard_C|GettileMap _output_get)) 1))
        (bind _output_get_2 (Variables|/Game/MyContent/Blueprints/Board/BP_ChessBoard.BP_ChessBoard_C|SetIndex (Variables|Default|GetChessBoardRef) _index))
        (if (and (.istilefree (.Value (Utilities|Map|Find (Variables|/Game/MyContent/Blueprints/Board/BP_ChessBoard.BP_ChessBoard_C|GettileMap (Variables|Default|GetChessBoardRef)) _output_get_2))) (.isspawntile (.Value (Utilities|Map|Find (Variables|/Game/MyContent/Blueprints/Board/BP_ChessBoard.BP_ChessBoard_C|GettileMap (Variables|Default|GetChessBoardRef)) _output_get_2))))
          (Rendering|Material|SetMaterial (.tilecomponentref (.Value (Utilities|Map|Find (Variables|/Game/MyContent/Blueprints/Board/BP_ChessBoard.BP_ChessBoard_C|GettileMap (Variables|Default|GetChessBoardRef)) _output_get_2))) 0 "/Game/MyContent/Materials/OverlayMAT/MAT_ObjectSelection.MAT_ObjectSelection")
          (Variables|PlayerCamera|SetCurrentCameraPosition "Board")
          (Variables|PlayerCamera|SetCameraInPosition false))))))

(event Custom|ManagingPawns
  (Variables|Default|SetCurrentPlayerState "NewEnumerator6")
  (Variables|PlayerCamera|SetCurrentCameraPosition "Board")
  (Variables|PlayerCamera|SetCameraInPosition false))

(event Custom|UpdateCamera
  (switch Utilities|FlowControl|Switch|SwitchonE_PlayerCameraStates (Variables|Default|GetCameraState)
    (:NewEnumerator0
      (CallFunction|CameraTableRotating))
    (:NewEnumerator1
      (CallFunction|CameraPointtoPointTransform))))

(event EventBeginPlay
  (bind _returnvalue (Game|GetPlayerController 0))
  (Variables|/Script/Engine.PlayerController|SetbShowMouseCursor _returnvalue true)
  (Variables|/Script/Engine.PlayerController|SetbEnableClickEvents _returnvalue true)
  (Variables|/Script/Engine.PlayerController|SetbEnableMouseOverEvents _returnvalue true)
  (Input|SetInputModeGameandUI _returnvalue 0 "DoNotLock" false false)
  (bind _returnvalue_2 (UserInterface|CreateWidget "/Game/MyContent/Blueprints/UserInterface/WB_ResourceCounter.WB_ResourceCounter_C"))
  (bind _output_get (Variables|Default|SetResourceCounterWBRef _returnvalue_2))
  (UserInterface|Viewport|AddtoViewport _output_get 0))

(event EventTick
  (params (DeltaSeconds :type Float%20%28single-precision%29))
  (CallFunction|UpdateCamera))

(event Input|KeyboardEvents|1
  (params (Key :type Key%20Structure :default "None"))
  ;[0 0 0 1 12] Event used for switching camera to next position.
  (:Pressed
    (CallFunction|CalcNextCameraPosition)
    (Variables|PlayerCamera|SetCanSwitchCamera false)
    (Variables|PlayerCamera|SetCameraInPosition false)))

(event Input|KeyboardEvents|2
  (params (Key :type Key%20Structure :default "None"))
  ;[0 0 0 1 12] Event used for toggling camera focus on a specific object.
  (:Pressed
    (Utilities|FlowControl|FlipFlop
      (:A
        (Variables|PlayerCamera|SetShouldFocusTarget true))
      (:B
        (Variables|PlayerCamera|SetShouldFocusTarget false)
        (Variables|PlayerCamera|SetCameraInPosition false)))))

(fn ConstructionScript
  (bind _keys (Utilities|Map|Keys (Variables|PlayerCamera|GetCameraPositions)))
  (for (_array_element _array_index) _keys
    (Utilities|Map|Add (Variables|PlayerCamera|GetCameraPositionFinder) _array_index _array_element)))

(fn CameraTableRotating
  (Components|Activation|SetActive (Variables|Default|GetRotatingCamera) true false)
  (Components|Activation|SetActive (Variables|Default|GetMainPlayerCamera) false false)
  (Transformation|SetRelativeRotation (Variables|Default|GetSpringArm) (Math|Rotator|MakeRotator 0.0 -3e+01 (+ (.yaw (Variables|/Script/Engine.SceneComponent|GetRelativeRotation (Variables|Default|GetSpringArm))) (* (Variables|Default|GetCameraRotationSpeed) (Utilities|Time|GetWorldDeltaSeconds)))) false false))

(fn CameraPointtoPointTransform
  (bind _returnvalue (Utilities|Time|GetWorldDeltaSeconds))
  (bind _returnvalue_2 (Utilities|Time|GetWorldDeltaSeconds))
  (bind _mainplayercamera (Variables|Default|GetMainPlayerCamera))
  (bind _cameratransitionspeed (Variables|PlayerCamera|GetCameraTransitionSpeed))
  (bind _cameratransitionspeed_2 (Variables|PlayerCamera|GetCameraTransitionSpeed))
  (bind _mainplayercamera_2 (Variables|Default|GetMainPlayerCamera))
  (bind _currentcameraposition (Variables|PlayerCamera|GetCurrentCameraPosition))
  (bind _camerapositions (Variables|PlayerCamera|GetCameraPositions))
  (bind _currentcameraposition_2 (Variables|PlayerCamera|GetCurrentCameraPosition))
  (bind _camerapositions_2 (Variables|PlayerCamera|GetCameraPositions))
  (bind _returnvalue_3 (Transformation|GetRelativeTransform _mainplayercamera))
  (bind _value (Utilities|Map|Find _camerapositions _currentcameraposition))
  (bind _value_2 (Utilities|Map|Find _camerapositions_2 _currentcameraposition_2))
  (bind _returnvalue_4 (* _returnvalue _cameratransitionspeed))
  (bind _returnvalue_5 (* _returnvalue_2 _cameratransitionspeed_2))
  (bind _relativelocation (Variables|/Script/Engine.SceneComponent|GetRelativeLocation _mainplayercamera_2))
  (bind _returnvalue_6 (Math|Float|Clamp(Float) _returnvalue_4))
  (bind _returnvalue_7 (Math|Float|Clamp(Float) _returnvalue_5))
  (bind _returnvalue_8 (Math|Vector|Lerp(Vector) _relativelocation (.location _value) _returnvalue_6))
  (bind _returnvalue_9 (Math|Transform|Lerp(Transform) _returnvalue_3 _value_2 _returnvalue_7))
  (Components|Activation|SetActive (Variables|Default|GetMainPlayerCamera) true false)
  (Components|Activation|SetActive (Variables|Default|GetRotatingCamera) false false)
  (if (Variables|PlayerCamera|GetShouldFocusTarget)
    (Utilities|IsValid (Variables|PlayerCamera|GetFocusTargetRef)
      (:Is%20Valid
        (Transformation|SetWorldRotation (Variables|Default|GetMainPlayerCamera) (Math|Rotator|Lerp(Rotator) (Transformation|GetWorldRotation (Variables|Default|GetMainPlayerCamera)) (Math|Rotator|FindLookatRotation (Transformation|GetWorldLocation (Variables|Default|GetMainPlayerCamera)) (Transformation|GetActorLocation (Variables|PlayerCamera|GetFocusTargetRef))) (Math|Float|Clamp(Float) (* (Utilities|Time|GetWorldDeltaSeconds) (Variables|PlayerCamera|GetCameraFollowSpeed)))) false false)
        (if (not (Variables|PlayerCamera|GetCameraInPosition))
          (Variables|PlayerCamera|SetTargetTransform (Math|Transform|MakeTransform _returnvalue_8 "0, 0, 0" "1.000000,1.000000,1.000000"))
          (if (Utilities|Operators|EqualEqual _returnvalue_8 (.location _value) 0.01)
            (Transformation|SetRelativeLocation (Variables|Default|GetMainPlayerCamera) (.location (.Value (Utilities|Map|Find (Variables|PlayerCamera|GetCameraPositions) (Variables|PlayerCamera|GetCurrentCameraPosition)))) false false)
            (else
              (Transformation|SetRelativeLocation (Variables|Default|GetMainPlayerCamera) (.location (Variables|PlayerCamera|GetTargetTransform)) false false)))
          (if (Utilities|Operators|EqualEqual (Variables|/Script/Engine.SceneComponent|GetRelativeLocation (Variables|Default|GetMainPlayerCamera)) (.location (.Value (Utilities|Map|Find (Variables|PlayerCamera|GetCameraPositions) (Variables|PlayerCamera|GetCurrentCameraPosition)))) 0.0)
            (Variables|PlayerCamera|SetCanSwitchCamera true)
            (Variables|PlayerCamera|SetCameraInPosition true)
            (else
              (Variables|PlayerCamera|SetCanSwitchCamera false)
              (Variables|PlayerCamera|SetCameraInPosition false)))))
      (:Is%20Not%20Valid
        (Development|PrintString "Focus Target Invalid")))
    (elif (not (Variables|PlayerCamera|GetCameraInPosition))
      (Variables|PlayerCamera|SetTargetTransform _returnvalue_9)
      (if (Class|KismetMathLibrary|NearlyEqualTransformTransform _returnvalue_9 _value_2 0.01 0.01 0.01)
        (Transformation|SetRelativeTransform (Variables|Default|GetMainPlayerCamera) (.Value (Utilities|Map|Find (Variables|PlayerCamera|GetCameraPositions) (Variables|PlayerCamera|GetCurrentCameraPosition))) false false)
        (else
          (Transformation|SetRelativeTransform (Variables|Default|GetMainPlayerCamera) (Variables|PlayerCamera|GetTargetTransform) false false)))
      (if (== (Transformation|GetRelativeTransform (Variables|Default|GetMainPlayerCamera)) (.Value (Utilities|Map|Find (Variables|PlayerCamera|GetCameraPositions) (Variables|PlayerCamera|GetCurrentCameraPosition))))
        (Variables|PlayerCamera|SetCanSwitchCamera true)
        (Variables|PlayerCamera|SetCameraInPosition true)
        (else
          (Variables|PlayerCamera|SetCanSwitchCamera false)
          (Variables|PlayerCamera|SetCameraInPosition false))))))