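; Chess board actor that builds a centred grid of tile meshes in its Construction Script, tinted green to blue by index.
; TileMap stores each tile's state, grid position, mesh and occupying pawn by index.
; Clicking traces under the cursor and spawns a BP_TestChessPiece on that tile if unoccupied.
; RegenerateTiles, not called here, rebuilds the grid preserving pawns, re-keys the map, trims surplus entries with their pawns and repositions the rest.
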(event EventBeginPlay)

(event MouseInput|EventActorOnClicked
  (params (ButtonPressed :type Key%20Structure))
  (CallFunction|AddPawn))

(fn ConstructionScript
  (CallFunction|SpawnInitialTiles))

(fn CalculateTilePos
  (Variables|BoardSize|SettilePos (Math|Vector|MakeVector (/ (- (* (/ (Variables|General|GetIndex) (Variables|BoardSize|GetboardCollumnLength)) (+ (Variables|BoardSize|GettileSize) (Variables|BoardSize|GettileSpacing))) (* (/ (- (Variables|BoardSize|GetboardRowLength) 1) 2) (+ (Variables|BoardSize|GettileSize) (Variables|BoardSize|GettileSpacing)))) -1.0) (- (* (Math|Integer|%(Integer) (Variables|General|GetIndex) (Variables|BoardSize|GetboardCollumnLength)) (+ (Variables|BoardSize|GettileSize) (Variables|BoardSize|GettileSpacing))) (* (/ (- (Variables|BoardSize|GetboardCollumnLength) 1) 2) (+ (Variables|BoardSize|GettileSize) (Variables|BoardSize|GettileSpacing)))) 0.0))
  (return (Math|Vector2D|MakeVector2D (Math|Conversions|ToFloat(Integer) (/ (Variables|General|GetIndex) (Variables|BoardSize|GetboardCollumnLength))) (Math|Conversions|ToFloat(Integer) (Math|Integer|%(Integer) (Variables|General|GetIndex) (Variables|BoardSize|GetboardCollumnLength))))))

(fn SpawnInitialTiles
  (for _index (range 0 (- (* (Variables|BoardSize|GetboardCollumnLength) (Variables|BoardSize|GetboardRowLength)) 1))
    (Variables|General|SetIndex _index)
    (bind _tile2dpos (CallFunction|CalculateTilePos))
    (LocalVariables|SetTile2dPos _tile2dpos)
    (bind _returnvalue (AddComponent|AddStaticMeshComponent false (Math|Transform|MakeTransform (Variables|BoardSize|GettilePos) "0, 0, 0" (Math|Conversions|ToVector(Float) (/ (Variables|BoardSize|GettileSize) 1e+02)))))
    (LocalVariables|SetstaticMeshCompRef _returnvalue)
    (Transformation|AttachComponentToComponent (LocalVariables|GetstaticMeshCompRef) (Variables|Default|GetDefaultSceneRoot) "None" "KeepRelative" "KeepRelative" "KeepRelative" true)
    (bind _returnvalue_2 (Rendering|Material|CreateDynamicMaterialInstance (LocalVariables|GetstaticMeshCompRef) 0 "/Game/MyContent/Materials/BasicMAT/MAT_DebugMaterial.MAT_DebugMaterial" "None" :!class /Script/Engine.PrimitiveComponent))
    (Rendering|Material|SetVectorParameterValue _returnvalue_2 "Colour" (Math|Color|Lerp(LinearColor) (Utilities|Struct|MakeLinearColor 0.0 1.0 0.0 1.0) (Utilities|Struct|MakeLinearColor 0.0 0.0 1.0 1.0) (/ (Variables|General|GetIndex) (- (* (Variables|BoardSize|GetboardCollumnLength) (Variables|BoardSize|GetboardRowLength)) 1))) :!class /Script/Engine.MaterialInstanceDynamic)
    (Utilities|Map|Add (Variables|BoardData|GettileMap) (Variables|General|GetIndex) (Utilities|Struct|MakeStr_BoardTileStructure true true 0 (LocalVariables|GetTile2dPos) (LocalVariables|GetstaticMeshCompRef)))))

(fn SortTileElements
  (LocalVariables|Setn (Utilities|Map|Length (Variables|BoardData|GettileMap)))
  (for _index (range 0 (- (LocalVariables|Getn) 1))
    (LocalVariables|Seti _index)
    (for _index_2 (range 0 (Utilities|Operators|Subtract (LocalVariables|Getn) 1 (LocalVariables|Geti)))
      (LocalVariables|Setj _index_2)
      (bind _keys (Utilities|Map|Keys (Variables|BoardData|GettileMap)))
      (if (> (Utilities|Array|Get(acopy) _keys (LocalVariables|Getj)) (Utilities|Array|Get(acopy) _keys (+ (LocalVariables|Getj) 1)))
        (bind _keys_2 (Utilities|Map|Keys (Variables|BoardData|GettileMap)))
        (Utilities|Array|Swap _keys_2 (LocalVariables|Getj) (+ (LocalVariables|Getj) 1)))))
  (Utilities|Map|Clear (Variables|BoardData|GettempTileMap))
  (bind _keys_3 (Utilities|Map|Keys (Variables|BoardData|GettileMap)))
  (for (_array_element _array_index) _keys_3
    (Utilities|Map|Add (Variables|BoardData|GettempTileMap) _array_index (.Value (Utilities|Map|Find (Variables|BoardData|GettileMap) _array_element))))
  (Utilities|Map|Clear (Variables|BoardData|GettileMap))
  (bind _keys_4 (Utilities|Map|Keys (Variables|BoardData|GettempTileMap)))
  (for (_array_element_2 _array_index_2) _keys_4
    (Utilities|Map|Add (Variables|BoardData|GettileMap) _array_index_2 (.Value (Utilities|Map|Find (Variables|BoardData|GettempTileMap) _array_element_2)))))

(fn AddPawn
  (bind _returnvalue (Game|GetPlayerController 0))
  (bind _hitresult (Game|Player|GetHitResultUnderCursorbyChannel _returnvalue "TraceTypeQuery1" true))
  (bind _values (Utilities|Map|Values (Variables|BoardData|GettileMap)))
  (for (_array_element _array_index) _values
    (Variables|General|SetIndex _array_index)
    (if (and (not (Utilities|IsValid (.occupiedpawn _array_element))) (== (.tilecomponentref _array_element) (.hitcomponent _hitresult)))
      (bind _returnvalue_2 (Game|SpawnActorfromClass "/Game/MyContent/Blueprints/Pawns/BP_TestChessPiece.BP_TestChessPiece_C" (Math|Transform|MakeTransform (Transformation|GetWorldLocation (.hitcomponent _hitresult)) "0, 0, 0" "1.000000,1.000000,1.000000") "AdjustIfPossibleButAlwaysSpawn" "MultiplyWithRoot" 0 0))
      (Utilities|Map|Add (Variables|BoardData|GettileMap) (Variables|General|GetIndex) (Utilities|Struct|MakeStr_BoardTileStructure (.istileactive (.Value (Utilities|Map|Find (Variables|BoardData|GettileMap) (Variables|General|GetIndex)))) (.istilefree (.Value (Utilities|Map|Find (Variables|BoardData|GettileMap) (Variables|General|GetIndex)))) _returnvalue_2 (.2dtilepos (.Value (Utilities|Map|Find (Variables|BoardData|GettileMap) (Variables|General|GetIndex)))) (.tilecomponentref (.Value (Utilities|Map|Find (Variables|BoardData|GettileMap) (Variables|General|GetIndex)))))))))

(fn RegenerateTiles
  (bind _tilemap (Variables|BoardData|GettileMap))
  (bind _tilemap_2 (Variables|BoardData|GettileMap))
  (bind _returnvalue (Utilities|Map|Length _tilemap_2))
  (bind _returnvalue_2 (- _returnvalue 1))
  (bind _value (Utilities|Map|Find _tilemap_2 _returnvalue_2))
  (for _index (range 0 (- (Utilities|Map|Length (Variables|BoardData|GettileMap)) 1))
    (Variables|General|SetIndex _index)
    (Utilities|IsValid (.tilecomponentref (.Value (Utilities|Map|Find (Variables|BoardData|GettileMap) (Variables|General|GetIndex))))
      (:Is%20Valid
        (Components|DestroyComponent (.tilecomponentref (.Value (Utilities|Map|Find (Variables|BoardData|GettileMap) (Variables|General|GetIndex))))))
      (:Is%20Not%20Valid
        (Development|PrintString "Invalid Tile"))))
  (for _index_2 (range 0 (- (* (Variables|BoardSize|GetboardCollumnLength) (Variables|BoardSize|GetboardRowLength)) 1))
    (Variables|General|SetIndex _index_2)
    (bind _tile2dpos (CallFunction|CalculateTilePos))
    (LocalVariables|SetTile2dPos _tile2dpos)
    (bind _returnvalue_3 (AddComponent|AddStaticMeshComponent false (Math|Transform|MakeTransform (Variables|BoardSize|GettilePos) "0, 0, 0" (Math|Conversions|ToVector(Float) (/ (Variables|BoardSize|GettileSize) 1e+02)))))
    (LocalVariables|SetstaticMeshCompRef _returnvalue_3)
    (Transformation|AttachComponentToComponent (LocalVariables|GetstaticMeshCompRef) (Variables|Default|GetDefaultSceneRoot) "None" "KeepRelative" "KeepRelative" "KeepRelative" true)
    (bind _returnvalue_4 (Rendering|Material|CreateDynamicMaterialInstance (LocalVariables|GetstaticMeshCompRef) 0 "/Game/MyContent/Materials/BasicMAT/MAT_DebugMaterial.MAT_DebugMaterial" "None" :!class /Script/Engine.PrimitiveComponent))
    (Rendering|Material|SetVectorParameterValue _returnvalue_4 "Colour" (Math|Color|Lerp(LinearColor) (Utilities|Struct|MakeLinearColor 0.0 1.0 0.0 1.0) (Utilities|Struct|MakeLinearColor 0.0 0.0 1.0 1.0) (/ (Variables|General|GetIndex) (- (* (Variables|BoardSize|GetboardCollumnLength) (Variables|BoardSize|GetboardRowLength)) 1))) :!class /Script/Engine.MaterialInstanceDynamic)
    (Utilities|Map|Add _tilemap (Variables|General|GetIndex) (Utilities|Struct|MakeStr_BoardTileStructure (.istileactive (.Value (Utilities|Map|Find _tilemap (Variables|General|GetIndex)))) (.istilefree (.Value (Utilities|Map|Find _tilemap (Variables|General|GetIndex)))) (.occupiedpawn (.Value (Utilities|Map|Find _tilemap (Variables|General|GetIndex)))) (LocalVariables|GetTile2dPos) (LocalVariables|GetstaticMeshCompRef))))
  (CallFunction|SortTileElements)
  (while (> (- (Utilities|Map|Length (Variables|BoardData|GettileMap)) 1) (- (* (Variables|BoardSize|GetboardCollumnLength) (Variables|BoardSize|GetboardRowLength)) 1))
    (Utilities|IsValid (.occupiedpawn _value)
      (:Is%20Valid
        (Actor|DestroyActor (.occupiedpawn _value)))
      (:Is%20Not%20Valid
        _))
    (Utilities|Map|Remove (Variables|BoardData|GettileMap) (- (Utilities|Map|Length (Variables|BoardData|GettileMap)) 1)))
  (CallFunction|RepositionPawns))

(fn DeleteAllTiles
  (CallFunction|SortTileElements)
  (for _index (range 0 (- (* (Variables|BoardSize|GetboardCollumnLength) (Variables|BoardSize|GetboardRowLength)) 1))
    (Variables|General|SetIndex _index)
    (Utilities|IsValid (.tilecomponentref (.Value (Utilities|Map|Find (Variables|BoardData|GettileMap) (Variables|General|GetIndex))))
      (:Is%20Valid
        (Components|DestroyComponent (.tilecomponentref (.Value (Utilities|Map|Find (Variables|BoardData|GettileMap) (Variables|General|GetIndex)))))
        (Utilities|Map|Remove (Variables|BoardData|GettileMap) (Variables|General|GetIndex)))
      (:Is%20Not%20Valid
        (Development|PrintString "Tile not vaild")))))

(fn RepositionPawns
  (for _index (range 0 (- (Utilities|Map|Length (Variables|BoardData|GettileMap)) 1))
    (Variables|General|SetIndex _index)
    (Utilities|IsValid (.occupiedpawn (.Value (Utilities|Map|Find (Variables|BoardData|GettileMap) (Variables|General|GetIndex))))
      (:Is%20Valid
        (Transformation|SetActorLocation (.occupiedpawn (.Value (Utilities|Map|Find (Variables|BoardData|GettileMap) (Variables|General|GetIndex)))) (Transformation|GetWorldLocation (.tilecomponentref (.Value (Utilities|Map|Find (Variables|BoardData|GettileMap) (Variables|General|GetIndex))))) false false)))))