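; BP_Card is a clickable card actor that holds one card's data and shows its name.
; Its construction script finds the BP_CardHand actor in the level and caches it as CardHandRef.
; PassHandtoCardData copies incoming card info, such as cost, images, stats and movement type, into CardData and updates the name text.
; Clicking the card calls RemoveCardMessage on the hand, passing itself.
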(event EventBeginPlay)

(event Collision|EventActorBeginOverlap
  (params (OtherActor :type Actor%20Object%20Reference)))

(event EventTick
  (params (DeltaSeconds :type Float%20%28single-precision%29)))

(event EventPassHandtoCardData
  (params (CardInfo :type Str%20Card%20Structure%20Structure))
  (bind _output_get (Variables|Default|SetCardData (Utilities|Struct|MakeStr_CardStructure (.cardname CardInfo) (.resoursecost CardInfo) (.characterimage CardInfo) (.cardactionsimage CardInfo) (.health CardInfo) (.attack CardInfo) (.speed CardInfo) (.movementtype CardInfo))))
  (Rendering|Components|TextRender|SetText (Variables|Default|GetCardName) (.cardname _output_get)))

(event MouseInput|EventActorOnClicked
  (params (ButtonPressed :type Key%20Structure :default "None"))
  (Class|BPICommonCardFunctions|RemoveCard(Message) (Variables|Default|GetCardHandRef) self))

(fn ConstructionScript
  (bind _returnvalue (Actor|GetActorOfClass "/Game/MyContent/Blueprints/Cards/BP_CardHand.BP_CardHand_C"))
  (Utilities|IsValid _returnvalue
    (:Is%20Valid
      (Variables|Default|SetCardHandRef _returnvalue))))