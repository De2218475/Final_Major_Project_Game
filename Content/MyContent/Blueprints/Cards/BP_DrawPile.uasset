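; BP_DrawPile is the draw pile that refills the player's card hand.
; On BeginPlay it caches the BP_CardHand and, if that exists, the LevelManager.
; DrawCards adds random monster cards until the hand reaches its max size, flagging it to reposition cards.
; If the hand is already full, it triggers the LevelManager's card burning event instead.
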(event Custom|DrawCards
  (bind _cardhandref (Variables|Default|GetCardHandRef))
  (bind _cardhandref_2 (Variables|Default|GetCardHandRef))
  (if (not (>= (Utilities|Map|Length (Variables|/Game/MyContent/Blueprints/Cards/BP_CardHand.BP_CardHand_C|GetCardList _cardhandref)) (Variables|/Game/MyContent/Blueprints/Cards/BP_CardHand.BP_CardHand_C|GetMaxHandSize _cardhandref)))
    (bind _output_get (Variables|Default|SetLastHandSize (Utilities|Operators|Subtract (Variables|/Game/MyContent/Blueprints/Cards/BP_CardHand.BP_CardHand_C|GetMaxHandSize _cardhandref_2) (Utilities|Map|Length (Variables|/Game/MyContent/Blueprints/Cards/BP_CardHand.BP_CardHand_C|GetCardList _cardhandref_2)) 1)))
    (for _index (range 0 _output_get)
      (Class|BPICommonCardFunctions|AddCardtoHand(Message) (Variables|Default|GetCardHandRef) (CallFunction|GetRandomMonsterCard))
      (Variables|/Game/MyContent/Blueprints/Cards/BP_CardHand.BP_CardHand_C|SetRepositioningCards? (Variables|Default|GetCardHandRef) true))
    (else
      (Default|CardBurningEvent (Variables|Default|GetLevelManager)))))

(event EventBeginPlay
  (bind _returnvalue (Actor|GetActorOfClass "/Game/MyContent/Blueprints/Cards/BP_CardHand.BP_CardHand_C"))
  (Utilities|IsValid _returnvalue
    (:Is%20Valid
      (Variables|Default|SetCardHandRef _returnvalue)
      (bind _returnvalue_2 (Actor|GetActorOfClass "/Game/MyContent/Blueprints/Gamemodes/TCGGamemode/SinglePlayer/GamemodeElements/LevelManager/LevelManager.LevelManager_C"))
      (Utilities|IsValid _returnvalue_2
        (:Is%20Valid
          (Variables|Default|SetLevelManager _returnvalue_2))))))

(event EventTick
  (params (DeltaSeconds :type Float%20%28single-precision%29)))

(fn ConstructionScript)