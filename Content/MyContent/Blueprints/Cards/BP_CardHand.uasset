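; BP_CardHand is the actor that holds the cards in hand and lays them out in a row centred on its location.
; Adding a card ID looks up its type in DT_MasterCardLibrary, spawns the Hero, Monster, Spell or Equipment card at the draw pile and passes its row data.
; CardList is re-indexed after changes; removal destroys the card and snaps the rest into place.
; While RepositioningCards is set, Tick lerps cards to their slots, calling LevelManager's CardBurningEvent on arrival.
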(event EventBeginPlay
  (Variables|CardPositioning|SetMiddlePoint (Transformation|GetActorLocation))
  (bind _returnvalue (Actor|GetActorOfClass "/Game/MyContent/Blueprints/Cards/BP_DrawPile.BP_DrawPile_C"))
  (Utilities|IsValid _returnvalue
    (:Is%20Valid
      (Variables|Default|SetDrawPileRef _returnvalue)
      (bind _returnvalue_2 (Actor|GetActorOfClass "/Game/MyContent/Blueprints/Gamemodes/TCGGamemode/SinglePlayer/GamemodeElements/LevelManager/LevelManager.LevelManager_C"))
      (Utilities|IsValid _returnvalue_2
        (:Is%20Valid
          (Variables|Default|SetLevelManagerRef _returnvalue_2))))))

(event EventTick
  (params (DeltaSeconds :type Float%20%28single-precision%29))
  (CallFunction|RepositionCardsInhand))

(event EventAddCardtoHand
  (params (CardID :type Name :default "None"))
  (CallFunction|LookUpandCreateCard CardID))

(event EventRemoveCardfromHand
  (params (RemovedCard :type Actor%20Object%20Reference))
  (Variables|General|SetRemoved%20Card RemovedCard)
  (for _index (range 0 (Utilities|Map|Length (Variables|Data|GetCardList)))
    (Variables|General|SetIndex _index)
    (if (== (Variables|General|GetRemoved%20Card) (.Value (Utilities|Map|Find (Variables|Data|GetCardList) _index)))
      (Utilities|Map|Remove (Variables|Data|GetCardList) (Variables|General|GetIndex))
      (Actor|DestroyActor (Variables|General|GetRemoved%20Card))))
  (CallFunction|SortMapElements)
  (for _index_2 (range 0 (Utilities|Map|Length (Variables|Data|GetCardList)))
    (Variables|General|SetIndex _index_2)
    (CallFunction|CalculateCardPos)
    (Utilities|IsValid (.Value (Utilities|Map|Find (Variables|Data|GetCardList) (Variables|General|GetIndex)))
      (:Is%20Valid
        (Transformation|SetActorLocation (.Value (Utilities|Map|Find (Variables|Data|GetCardList) (Variables|General|GetIndex))) (Variables|CardPositioning|GetCardPos) false false)))))

(fn ConstructionScript)

(fn LookUpandCreateCard
  (params (CardID :type Name))
  (bind _cardlist (Variables|Data|GetCardList))
  (bind _output_get (LocalVariables|SetfoundCardID CardID))
  (bind _returnvalue (Utilities|GetDataTableRow "/Game/MyContent/Blueprints/Cards/CardData/DataTables/DT_MasterCardLibrary.DT_MasterCardLibrary" _output_get)
    (:then
      (if (Utilities|Enum|Equal(Enum) (.cardidtype _returnvalue) "H")
        (LocalVariables|SetfoundCardType "NewEnumerator0")
        (switch Utilities|FlowControl|Switch|SwitchonE_CardTypes (LocalVariables|GetfoundCardType) :!label _label
          (:NewEnumerator0
            (bind _returnvalue_2 (Utilities|GetDataTableRow "/Game/MyContent/Blueprints/Cards/CardData/DataTables/HeroCardDTs/DT_HeroCardLibrary.DT_HeroCardLibrary" (LocalVariables|GetfoundCardID))
              (:then
                (LocalVariables|SetHeroCardStruct _returnvalue_2)
                (bind _returnvalue_3 (Game|SpawnActorfromClass "/Game/MyContent/Blueprints/Cards/CardBaseBPs/BP_HeroCard.BP_HeroCard_C" (Math|Transform|MakeTransform (+ (Transformation|GetActorLocation (Variables|Default|GetDrawPileRef)) "0.000000,0.000000,5.000000") (Transformation|GetActorRotation) "1.000000,1.000000,1.000000") "Undefined" "MultiplyWithRoot" 0 0))
                (Variables|General|SetAddedCard _returnvalue_3))))
          (:NewEnumerator1
            (bind _returnvalue_4 (Utilities|GetDataTableRow "/Game/MyContent/Blueprints/Cards/CardData/DataTables/MonsterCardDTs/DT_MonsterCardLibrary.DT_MonsterCardLibrary" (LocalVariables|GetfoundCardID))
              (:then
                (LocalVariables|SetMonsterCardStruct _returnvalue_4)
                (bind _returnvalue_5 (Game|SpawnActorfromClass "/Game/MyContent/Blueprints/Cards/CardBaseBPs/BP_MonsterCard.BP_MonsterCard_C" (Math|Transform|MakeTransform (+ (Transformation|GetActorLocation (Variables|Default|GetDrawPileRef)) "0.000000,0.000000,5.000000") (Transformation|GetActorRotation) "1.000000,1.000000,1.000000") "Undefined" "MultiplyWithRoot" 0 0))
                (Variables|General|SetAddedCard _returnvalue_5))))
          (:NewEnumerator2
            (bind _returnvalue_6 (Utilities|GetDataTableRow "/Game/MyContent/Blueprints/Cards/CardData/DataTables/SpellCardDTs/DT_SpellCardLibrary.DT_SpellCardLibrary" (LocalVariables|GetfoundCardID))
              (:then
                (LocalVariables|SetSpellCardStruct _returnvalue_6)
                (bind _returnvalue_7 (Game|SpawnActorfromClass "/Game/MyContent/Blueprints/Cards/CardBaseBPs/BP_SpellCard.BP_SpellCard_C" (Math|Transform|MakeTransform (+ (Transformation|GetActorLocation (Variables|Default|GetDrawPileRef)) "0.000000,0.000000,5.000000") (Transformation|GetActorRotation) "1.000000,1.000000,1.000000") "Undefined" "MultiplyWithRoot" 0 0))
                (Variables|General|SetAddedCard _returnvalue_7))))
          (:NewEnumerator3
            (bind _returnvalue_8 (Utilities|GetDataTableRow "/Game/MyContent/Blueprints/Cards/CardData/DataTables/EquipmentCardDTs/DT_EquipmentCardLibrary.DT_EquipmentCardLibrary" (LocalVariables|GetfoundCardID))
              (:then
                (LocalVariables|SetEquipmentCardStruct _returnvalue_8)
                (bind _returnvalue_9 (Game|SpawnActorfromClass "/Game/MyContent/Blueprints/Cards/CardBaseBPs/BP_EquipmentCard.BP_EquipmentCard_C" (Math|Transform|MakeTransform (+ (Transformation|GetActorLocation (Variables|Default|GetDrawPileRef)) "0.000000,0.000000,5.000000") (Transformation|GetActorRotation) "1.000000,1.000000,1.000000") "Undefined" "MultiplyWithRoot" 0 0))
                (Variables|General|SetAddedCard _returnvalue_9)))))
        (Utilities|Map|Add _cardlist (+ (Utilities|Map|Length _cardlist) 1) (Variables|General|GetAddedCard))
        (CallFunction|SortMapElements)
        (switch Utilities|FlowControl|Switch|SwitchonE_CardTypes (LocalVariables|GetfoundCardType)
          (:NewEnumerator0
            (Class|BPICommonCardFunctions|PassDatatoHeroCard(Message) (Variables|General|GetAddedCard) (LocalVariables|GetHeroCardStruct)))
          (:NewEnumerator1
            (Class|BPICommonCardFunctions|PassDatatoMonsterCard(Message) (Variables|General|GetAddedCard) (LocalVariables|GetMonsterCardStruct)))
          (:NewEnumerator2
            (Class|BPICommonCardFunctions|PassDatatoSpellCard(Message) (Variables|General|GetAddedCard) (LocalVariables|GetSpellCardStruct)))
          (:NewEnumerator3
            (Class|BPICommonCardFunctions|PassDatatoEquipmentCard(Message) (Variables|General|GetAddedCard) (LocalVariables|GetEquipmentCardStruct))))
        (elif (Utilities|Enum|Equal(Enum) (.cardidtype _returnvalue) "M")
          (LocalVariables|SetfoundCardType "NewEnumerator1")
          (goto _label)
          (elif (Utilities|Enum|Equal(Enum) (.cardidtype _returnvalue) "S")
            (LocalVariables|SetfoundCardType "NewEnumerator2")
            (goto _label)
            (elif (Utilities|Enum|Equal(Enum) (.cardidtype _returnvalue) "E")
              (LocalVariables|SetfoundCardType "NewEnumerator3")
              (goto _label)
              (else
                (Development|PrintString "IDType_Invalid")))))))))

(fn CalculateCardPos
  (Variables|CardPositioning|SetCardPos (+ (Variables|CardPositioning|GetMiddlePoint) (* (* (- (Variables|General|GetIndex) (/ (- (Utilities|Map|Length (Variables|Data|GetCardList)) 1) 2.0)) (+ (Variables|CardPositioning|GetCardWidth) (Variables|CardPositioning|GetCardSpacing))) (Variables|CardPositioning|GetDirection)))))

(fn SortMapElements
  (LocalVariables|Setn (Utilities|Map|Length (Variables|Data|GetCardList)))
  (for _index (range 0 (- (LocalVariables|Getn) 1))
    (LocalVariables|Seti _index)
    (for _index_2 (range 0 (Utilities|Operators|Subtract (LocalVariables|Getn) 1 (LocalVariables|Geti)))
      (LocalVariables|Setj _index_2)
      (bind _keys (Utilities|Map|Keys (Variables|Data|GetCardList)))
      (if (> (Utilities|Array|Get(acopy) _keys (LocalVariables|Getj)) (Utilities|Array|Get(acopy) _keys (+ (LocalVariables|Getj) 1)))
        (bind _keys_2 (Utilities|Map|Keys (Variables|Data|GetCardList)))
        (Utilities|Array|Swap _keys_2 (LocalVariables|Getj) (+ (LocalVariables|Getj) 1)))))
  (Utilities|Map|Clear (Variables|Data|GetTempMap))
  (bind _keys_3 (Utilities|Map|Keys (Variables|Data|GetCardList)))
  (for (_array_element _array_index) _keys_3
    (Utilities|Map|Add (Variables|Data|GetTempMap) _array_index (.Value (Utilities|Map|Find (Variables|Data|GetCardList) _array_element))))
  (Utilities|Map|Clear (Variables|Data|GetCardList))
  (bind _keys_4 (Utilities|Map|Keys (Variables|Data|GetTempMap)))
  (for (_array_element_2 _array_index_2) _keys_4
    (Utilities|Map|Add (Variables|Data|GetCardList) _array_index_2 (.Value (Utilities|Map|Find (Variables|Data|GetTempMap) _array_element_2)))))

(fn RepositionCardsInhand
  (if (Variables|Default|GetRepositioningCards?)
    (for _index (range 0 (- (Utilities|Map|Length (Variables|Data|GetCardList)) 1))
      (Variables|General|SetIndex _index)
      (CallFunction|CalculateCardPos)
      (Variables|Default|SetLastCardPos (Transformation|GetActorLocation (.Value (Utilities|Map|Find (Variables|Data|GetCardList) (Variables|General|GetIndex)))))
      (if (Utilities|Operators|EqualEqual (Variables|Default|GetLastCardPos) (Variables|CardPositioning|GetCardPos) 0.01)
        (Variables|Default|SetRepositioningCards? false)
        (Default|CardBurningEvent (Variables|Default|GetLevelManagerRef))
        (else
          (Transformation|SetActorLocation (.Value (Utilities|Map|Find (Variables|Data|GetCardList) (Variables|General|GetIndex))) (Math|Vector|Lerp(Vector) (Variables|Default|GetLastCardPos) (Variables|CardPositioning|GetCardPos) (Math|Float|Clamp(Float) (* (Utilities|Time|GetWorldDeltaSeconds) 5.0))) false false))))))