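; Base playing card actor for a TCG, handling click selection during the card burning and card playing match phases.
; On click, it reads the LevelManager's match state, sets the player's state, and replaces any open burn or play widget with a new one referencing this card.
; It then highlights only itself among all cards.
; PlayCard and BurnCard are empty events, and the construction script caches the card hand.
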(event Custom|PlayCard)

(event Custom|BurnCard)

(event EventBeginPlay
  (bind _returnvalue (Actor|GetActorOfClass "/Game/MyContent/Blueprints/Gamemodes/TCGGamemode/SinglePlayer/GamemodeElements/LevelManager/LevelManager.LevelManager_C"))
  (Utilities|IsValid _returnvalue
    (:Is%20Valid
      (Variables|Default|SetLevelManagerRef _returnvalue)
      (bind _asbp_tcgplayer (Utilities|Casting|CastToBP_TCGPlayer (Game|Player|GetPlayerPawn 0)))
      (Variables|Default|SetAs%20BP%20TCGPlayer _asbp_tcgplayer))))

(event MouseInput|EventActorOnClicked
  (params (ButtonPressed :type Key%20Structure))
  (bind _as_bp_tcgplayer (Variables|Default|GetAs%20BP%20TCGPlayer))
  (switch Utilities|FlowControl|Switch|SwitchonE_MatchStates (Variables|/Game/MyContent/Blueprints/Gamemodes/TCGGamemode/SinglePlayer/GamemodeElements/LevelManager/LevelManager.LevelManager_C|GetMatchStates (Variables|Default|GetLevelManagerRef))
    (:NewEnumerator1
      (Variables|/Game/MyContent/Blueprints/Gamemodes/TCGGamemode/SinglePlayer/PlayerRelated/BP_TCGPlayer.BP_TCGPlayer_C|SetCurrentPlayerState _as_bp_tcgplayer "NewEnumerator2")
      (bind _foundwidgets (Widget|GetAllWidgetsOfClass "/Game/MyContent/Blueprints/UserInterface/WB_BurnCard.WB_BurnCard_C" false))
      (for _array_element _foundwidgets
        (Utilities|IsValid _array_element
          (:Is%20Valid
            (Widget|RemovefromParent _array_element))))
      (bind _returnvalue (UserInterface|CreateWidget "/Game/MyContent/Blueprints/UserInterface/WB_BurnCard.WB_BurnCard_C" (Game|GetPlayerController 0)))
      (bind _output_get (Variables|Default|SetBurnCardWidgetRef _returnvalue))
      (UserInterface|Viewport|AddtoViewport _output_get 0)
      (Variables|/Game/MyContent/Blueprints/UserInterface/WB_BurnCard.WB_BurnCard_C|SetCardRef _returnvalue self))
    (:NewEnumerator2
      (Variables|/Game/MyContent/Blueprints/Gamemodes/TCGGamemode/SinglePlayer/PlayerRelated/BP_TCGPlayer.BP_TCGPlayer_C|SetCurrentPlayerState _as_bp_tcgplayer "NewEnumerator5")
      (bind _foundwidgets_2 (Widget|GetAllWidgetsOfClass "/Game/MyContent/Blueprints/UserInterface/WB_PlayCard.WB_PlayCard_C" false))
      (for _array_element_2 _foundwidgets_2
        (Utilities|IsValid _array_element_2
          (:Is%20Valid
            (Widget|RemovefromParent _array_element_2))))
      (bind _returnvalue_2 (UserInterface|CreateWidget "/Game/MyContent/Blueprints/UserInterface/WB_PlayCard.WB_PlayCard_C" (Game|GetPlayerController 0)))
      (bind _output_get_2 (Variables|Default|SetPlayCardWidgetRef _returnvalue_2))
      (UserInterface|Viewport|AddtoViewport _output_get_2 0)
      (Variables|/Game/MyContent/Blueprints/UserInterface/WB_PlayCard.WB_PlayCard_C|SetCardRef _returnvalue_2 self)))
  (bind _outactors (Actor|GetAllActorsOfClass "BP_BasePlayingCard_C"))
  (for _array_element_3 _outactors
    (Development|SetHiddeninGame (Variables|BP_BasePlayingCard_C|GetCardHighlight _array_element_3) true false))
  (Development|SetHiddeninGame (Variables|Default|GetCardHighlight) false false))

(fn ConstructionScript
  (bind _returnvalue (Actor|GetActorOfClass "/Game/MyContent/Blueprints/Cards/BP_CardHand.BP_CardHand_C"))
  (Utilities|IsValid _returnvalue
    (:Is%20Valid
      (Variables|Default|SetCardHandRef _returnvalue))))