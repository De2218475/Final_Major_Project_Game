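; Base Blueprint for a clickable hero card actor that belongs to a card hand.
; The construction script finds the BP_CardHand actor in the level and caches a reference to it.
; A data-passing event stores the hero card data and writes the card name to its text.
; Clicking the card sends the hand a message to remove it.
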(event EventBeginPlay)

(event EventPassDatatoHeroCard
  (params (HeroCardData :type Str%20Base%20Hero%20Card%20Structure%20Structure))
  (bind _output_get (Variables|Default|SetHeroCardData HeroCardData))
  (Rendering|Components|TextRender|SetText (Variables|Default|GetCardName) (.cardname _output_get)))

(event MouseInput|EventActorOnClicked
  (params (ButtonPressed :type Key%20Structure :default "None"))
  (Class|BPICommonCardFunctions|RemoveCardfromHand(Message) (Variables|Default|GetCardHandRef) self))

(fn ConstructionScript
  (bind _returnvalue (Actor|GetActorOfClass "/Game/MyContent/Blueprints/Cards/BP_CardHand.BP_CardHand_C"))
  (Utilities|IsValid _returnvalue
    (:Is%20Valid
      (Variables|Default|SetCardHandRef _returnvalue))))