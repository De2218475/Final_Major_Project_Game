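; BP_HeroCard is the hero card Blueprint for a card game, letting the player play a hero from the hand.
; PassDatatoHeroCard stores the hero data and sets the displayed card name.
; PlayCard closes the selection widget, writes the card's identity into BP_TCGPlayer's PlayerData while keeping resource points, and calls PlacingPawn.
; It then messages the hand to remove the card.
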(event EventBeginPlay
  (|CallParentFunction) ; This node is disabled and will not be called.\nDrag off pins to build functionality.
)

(event EventPlayCard
  (bind _herocarddata (Variables|Default|GetHeroCardData))
  (Widget|RemovefromParent (Variables|Default|GetCardPlaySelectionWB))
  (bind _asbp_tcgplayer (Utilities|Casting|CastToBP_TCGPlayer (Game|Player|GetPlayerPawn 0)))
  (bind _output_get (Variables|Default|SetAs%20BP%20TCGPlayer _asbp_tcgplayer))
  (Variables|/Game/MyContent/Blueprints/Gamemodes/TCGGamemode/SinglePlayer/BP_TCGPlayer.BP_TCGPlayer_C|SetPlayerData _output_get (Utilities|Struct|MakeStr_PlayerData (Utilities|Struct|MakeStr_BaseCardStructure (.cardidtype _herocarddata) (.cardidindex _herocarddata) (.cardname _herocarddata)) (.resourcepoints (Variables|/Game/MyContent/Blueprints/Gamemodes/TCGGamemode/SinglePlayer/BP_TCGPlayer.BP_TCGPlayer_C|GetPlayerData _output_get))))
  (Default|PlacingPawn (Variables|Default|GetAs%20BP%20TCGPlayer))
  (Class|BPICommonCardFunctions|RemoveCardfromHand(Message) (Variables|Default|GetCardHandRef) self))

(event EventPassDatatoHeroCard
  (params (HeroCardData :type Str%20Base%20Hero%20Card%20Structure%20Structure))
  (bind _output_get (Variables|Default|SetHeroCardData HeroCardData))
  (Rendering|Components|TextRender|SetText (Variables|Default|GetCardName) (.cardname _output_get)))

(fn ConstructionScript
  (|CallParentFunction))