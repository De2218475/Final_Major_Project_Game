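; BP_MonsterCard is the monster card Blueprint in a TCG, with logic to be played or burned.
; It receives MonsterCardData and builds its card widget from the name and character image.
; Playing checks resource points, then either deducts cost, records the selected card, starts pawn placement and messages the hand to remove it, or shows an insufficient-points widget.
; Burning grants one resource point and refreshes the counter, without removing the card from the hand here.
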(event EventBeginPlay
  (|CallParentFunction) ; This node is disabled and will not be called.\nDrag off pins to build functionality.
)

(event EventPlayCard
  (bind _monstercarddata (Variables|Default|GetMonsterCardData))
  (Widget|RemovefromParent (Variables|Default|GetPlayCardWidgetRef))
  (bind _asbp_tcgplayer (Utilities|Casting|CastToBP_TCGPlayer (Game|Player|GetPlayerPawn 0)))
  (Variables|Default|SetAs%20BP%20TCGPlayer _asbp_tcgplayer)
  (if (>= (.resourcepoints (Variables|/Game/MyContent/Blueprints/Gamemodes/TCGGamemode/SinglePlayer/BP_TCGPlayer.BP_TCGPlayer_C|GetPlayerData (Variables|Default|GetAs%20BP%20TCGPlayer))) (.cardresourcecost (Variables|Default|GetMonsterCardData)))
    (Variables|/Game/MyContent/Blueprints/Gamemodes/TCGGamemode/SinglePlayer/BP_TCGPlayer.BP_TCGPlayer_C|SetPlayerData (Variables|Default|GetAs%20BP%20TCGPlayer) (Utilities|Struct|MakeStr_PlayerData (Utilities|Struct|MakeStr_BaseCardStructure (.cardidtype _monstercarddata) (.cardidindex _monstercarddata) (.cardname _monstercarddata)) (- (.resourcepoints (Variables|/Game/MyContent/Blueprints/Gamemodes/TCGGamemode/SinglePlayer/BP_TCGPlayer.BP_TCGPlayer_C|GetPlayerData (Variables|Default|GetAs%20BP%20TCGPlayer))) (.cardresourcecost (Variables|Default|GetMonsterCardData)))))
    (Default|PlacingPawn (Variables|Default|GetAs%20BP%20TCGPlayer))
    (Class|BPICommonCardFunctions|RemoveCardfromHand(Message) (Variables|Default|GetCardHandRef) self)
    (else
      (bind _returnvalue (UserInterface|CreateWidget "/Game/MyContent/Blueprints/UserInterface/WB_InsufficientRP.WB_InsufficientRP_C" (Game|GetPlayerController 0)))
      (UserInterface|Viewport|AddtoViewport _returnvalue 0))))

(event EventBurnCard
  (Widget|RemovefromParent (Variables|Default|GetBurnCardWidgetRef))
  (bind _asbp_tcgplayer (Utilities|Casting|CastToBP_TCGPlayer (Game|Player|GetPlayerPawn 0)))
  (bind _output_get (Variables|Default|SetAs%20BP%20TCGPlayer _asbp_tcgplayer))
  (Variables|/Game/MyContent/Blueprints/Gamemodes/TCGGamemode/SinglePlayer/BP_TCGPlayer.BP_TCGPlayer_C|SetPlayerData (Variables|Default|GetAs%20BP%20TCGPlayer) (Utilities|Struct|MakeStr_PlayerData (.cardselected (Variables|/Game/MyContent/Blueprints/Gamemodes/TCGGamemode/SinglePlayer/BP_TCGPlayer.BP_TCGPlayer_C|GetPlayerData _output_get)) (+ (.resourcepoints (Variables|/Game/MyContent/Blueprints/Gamemodes/TCGGamemode/SinglePlayer/BP_TCGPlayer.BP_TCGPlayer_C|GetPlayerData _output_get)) 1)))
  (Default|UpdateResourcePointCounter (Variables|/Game/MyContent/Blueprints/Gamemodes/TCGGamemode/SinglePlayer/BP_TCGPlayer.BP_TCGPlayer_C|GetResourceCounterWBRef (Variables|Default|GetAs%20BP%20TCGPlayer))))

(event EventPassDatatoMonsterCard
  (params (MonsterCardData :type Str%20Base%20Monster%20Card%20Structure%20Structure))
  (bind _output_get (Variables|Default|SetMonsterCardData MonsterCardData))
  (bind _returnvalue (UserInterface|CreateWidget "/Game/MyContent/Blueprints/Cards/Widgets/CardTemplates/BP_MonsterCardWidget.BP_MonsterCardWidget_C" 0 (.cardname _output_get) (.cardcharacterimage _output_get)))
  (UserInterface|SetWidget (Variables|Default|GetCardWidget) _returnvalue))

(fn ConstructionScript
  (|CallParentFunction))