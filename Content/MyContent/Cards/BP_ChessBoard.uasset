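; BP_ChessBoard is an actor that spawns cube tiles at BeginPlay, one per cell of the column-by-row board size.
; Each half-scale cube component is placed at the position CalculateTilePos computes from the loop index, tile size and actor location.
; That offset applies equally to X, Y and Z, so tiles follow a diagonal rather than a grid.
; Each computed position is printed for debugging.
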(event EventBeginPlay
  (for _index (range 0 (- (* (Variables|Default|GetboardCollumnLength) (Variables|Default|GetboardRowLength)) 1))
    (Variables|Default|SetIndex _index)
    (CallFunction|CalculateTilePos)
    (bind _returnvalue (AddComponent|AddStaticMeshComponent false (Math|Transform|MakeTransform "0, 0, 0" "0, 0, 0" "0.500000,0.500000,0.500000")))
    (Components|StaticMesh|SetStaticMesh _returnvalue "/Game/StarterContent/Shapes/Shape_Cube.Shape_Cube")
    (Transformation|SetWorldLocation _returnvalue (Variables|Default|GettilePos) false false)))

(event Collision|EventActorBeginOverlap
  (params (OtherActor :type Actor%20Object%20Reference)))

(event EventTick
  (params (DeltaSeconds :type Float%20%28single-precision%29)))

(fn ConstructionScript)

(fn CalculateTilePos
  (bind _output_get (Variables|Default|SettilePos (+ (* (* (/ (Variables|Default|GetIndex) 2) (* (Variables|Default|GettileSize) 2.0)) (Math|Vector|MakeVector 1.0 1.0 1.0)) (Transformation|GetActorLocation))))
  (Development|PrintString (Utilities|String|ToString(Vector) _output_get)))