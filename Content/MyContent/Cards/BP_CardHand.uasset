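; Card hand actor that spawns, removes and lays out named cards in a row centred around its starting location.
; AddCard and RemoveCard maintain an index-to-card map, repositioning cards through CalculateCardPos using width, spacing and a direction vector.
; On removal, SortMapElements rebuilds the map with consecutive zero-based keys via a temporary map, whereas AddCard inserts at length plus one.
; Its bubble-sort pass only swaps copied key arrays, leaving the order unchanged.
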(event EventBeginPlay
  (Variables|Default|SetMiddlePoint (Transformation|GetActorLocation)))

(event EventTick
  (params (DeltaSeconds :type Float%20%28single-precision%29)))

(event EventAddCard
  (params (CardInfo :type Str%20Card%20Structure%20Structure))
  (bind _cardlist (Variables|Default|GetCardList))
  (bind _returnvalue (Utilities|Map|Length _cardlist))
  (Variables|Default|SetCard%20Info%20Card%20Name (.cardname CardInfo))
  (bind _returnvalue_2 (Game|SpawnActorfromClass "/Game/MyContent/Cards/Card.Card_C" (Math|Transform|MakeTransform "0, 0, 0" (Math|Rotator|MakeRotator 0.0 0.0 (.yaw (Transformation|GetActorRotation))) "1.000000,1.000000,1.000000") "Undefined" "MultiplyWithRoot" 0 0))
  (Rendering|Components|TextRender|SetText (Variables|/Game/MyContent/Cards/Card.Card_C|GetCardName _returnvalue_2) (Variables|Default|GetCard%20Info%20Card%20Name))
  (Utilities|Map|Add _cardlist (+ _returnvalue 1) _returnvalue_2)
  (Development|PrintString (Utilities|String|ToString(Integer) _returnvalue))
  (for _index (range 0 (Utilities|Map|Length (Variables|Default|GetCardList)))
    (Variables|Default|SetIndex _index)
    (CallFunction|CalculateCardPos)
    (Utilities|IsValid (.Value (Utilities|Map|Find (Variables|Default|GetCardList) (Variables|Default|GetIndex)))
      (:Is%20Valid
        (Transformation|SetActorLocation (.Value (Utilities|Map|Find (Variables|Default|GetCardList) (Variables|Default|GetIndex))) (Variables|Default|GetCardPos) false false)))))

(event EventRemoveCard
  (params (RemovedCard :type Actor%20Object%20Reference))
  (Variables|Default|SetRemoved%20Card RemovedCard)
  (for _index (range 0 (Utilities|Map|Length (Variables|Default|GetCardList)))
    (Variables|Default|SetIndex _index)
    (if (== (Variables|Default|GetRemoved%20Card) (.Value (Utilities|Map|Find (Variables|Default|GetCardList) _index)))
      (Utilities|Map|Remove (Variables|Default|GetCardList) (Variables|Default|GetIndex))
      (Actor|DestroyActor (Variables|Default|GetRemoved%20Card))
      (CallFunction|SortMapElements)
      (CallFunction|CalculateCardPos))
    (for _index_2 (range 0 (Utilities|Map|Length (Variables|Default|GetCardList)))
      (Variables|Default|SetIndex _index_2)
      (CallFunction|CalculateCardPos)
      (Utilities|IsValid (.Value (Utilities|Map|Find (Variables|Default|GetCardList) (Variables|Default|GetIndex)))
        (:Is%20Valid
          (Transformation|SetActorLocation (.Value (Utilities|Map|Find (Variables|Default|GetCardList) (Variables|Default|GetIndex))) (Variables|Default|GetCardPos) false false)))))
  (Development|PrintString (Utilities|String|Append "Card List Len: " (Utilities|String|ToString(Integer) (Utilities|Map|Length (Variables|Default|GetCardList)))))
  (Development|PrintString (Utilities|String|Append "Index: " (Utilities|String|ToString(Integer) (Variables|Default|GetIndex)))))

(fn ConstructionScript)

(fn CalculateCardPos
  (bind _cardwidth (Variables|Default|GetCardWidth))
  (bind _cardspacing (Variables|Default|GetCardSpacing))
  (bind _returnvalue (+ _cardwidth _cardspacing))
  (Variables|Default|SetCardPos (+ (Variables|Default|GetMiddlePoint) (* (- (* (- (Variables|Default|GetIndex) (/ (- (Utilities|Map|Length (Variables|Default|GetCardList)) 1) 2.0)) _returnvalue) _returnvalue) (Variables|Default|GetDirection)))))

(fn SortMapElements
  (LocalVariables|Setn (Utilities|Map|Length (Variables|Default|GetCardList)))
  (for _index (range 0 (- (LocalVariables|Getn) 1))
    (LocalVariables|Seti _index)
    (for _index_2 (range 0 (Utilities|Operators|Subtract (LocalVariables|Getn) 1 (LocalVariables|Geti)))
      (LocalVariables|Setj _index_2)
      (bind _keys (Utilities|Map|Keys (Variables|Default|GetCardList)))
      (if (> (Utilities|Array|Get(acopy) _keys (LocalVariables|Getj)) (Utilities|Array|Get(acopy) _keys (+ (LocalVariables|Getj) 1)))
        (bind _keys_2 (Utilities|Map|Keys (Variables|Default|GetCardList)))
        (Utilities|Array|Swap _keys_2 (LocalVariables|Getj) (+ (LocalVariables|Getj) 1)))))
  (Utilities|Map|Clear (Variables|Default|GetTempMap))
  (bind _keys_3 (Utilities|Map|Keys (Variables|Default|GetCardList)))
  (for (_array_element _array_index) _keys_3
    (Utilities|Map|Add (Variables|Default|GetTempMap) _array_index (.Value (Utilities|Map|Find (Variables|Default|GetCardList) _array_element))))
  (Utilities|Map|Clear (Variables|Default|GetCardList))
  (bind _keys_4 (Utilities|Map|Keys (Variables|Default|GetTempMap)))
  (for (_array_element_2 _array_index_2) _keys_4
    (Utilities|Map|Add (Variables|Default|GetCardList) _array_index_2 (.Value (Utilities|Map|Find (Variables|Default|GetTempMap) _array_element_2)))))